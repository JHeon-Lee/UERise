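; BP_IconText is a short-lived world actor that shows two text fields and an icon through a WBP_IconText widget, part of a custom damage and status text set.
; On BeginPlay it pushes colors, fonts (with a default fallback), icon and size, and texts into the widget.
; Optional distance scaling shrinks the widget beyond a minimum distance from the player pawn, computed once at spawn.
; It then plays the chosen animation and destroys itself after the on-screen time.
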(event EventBeginPlay
  (bind _returnvalue (Game|Player|GetPlayerPawn 0))
  (bind _font (Variables|Default|GetFont))
  (bind _font_2 (Variables|Default|GetFont%202))
  (bind _timeonscreen (Variables|Default|GetTimeOnScreen))
  (bind _scaleminimumdistance (Variables|Default|GetScaleMinimumDistance))
  (bind _widget (Variables|Default|GetWidget))
  (bind _returnvalue_2 (Transformation|GetWorldLocation _widget))
  (bind _returnvalue_3 (Transformation|GetActorLocation _returnvalue))
  (bind _returnvalue_4 (Math|Vector|Distance(Vector) _returnvalue_2 _returnvalue_3))
  (bind _returnvalue_5 (/ _scaleminimumdistance _returnvalue_4))
  (Utilities|FlowControl|Sequence
    (:then_0
      ;[1 1 1] Creating a widget reference to call functions
      (bind _aswbp_icon_text (Utilities|Casting|CastToWBP_IconText (UserInterface|GetUserWidgetObject (Variables|Default|GetWidget))))
      (Variables|Default|SetWBP_IconText%20Reference _aswbp_icon_text))
    (:then_1
      ;[1 1 1] Changes widget font color
      (Default|ChangeFontColorandOpacity (Variables|Default|GetWBP_IconText%20Reference) (Variables|Default|GetColor))
      (Default|ChangeSecondTextFontColorandOpacity (Variables|Default|GetWBP_IconText%20Reference) (Variables|Default|GetColor2)))
    (:then_2
      ;[1 1 1] Gets Icon from macro and sends it to WBP_IconText
      (Default|ChangeIcon (Variables|Default|GetWBP_IconText%20Reference) (Variables|Default|GetIcon)))
    (:then_3
      ;[1 1 1] Check if font is valid and then changes it. If font is not valid or not selected, it defaults to ROBOTO
      (Default|ChangeFontText (Variables|Default|GetWBP_IconText%20Reference) (select (Utilities|IsValid (.FontObject (Utilities|Struct|BreakSlateFontInfo _font))) _font (Variables|Default|GetDefaultFont)))
      (Default|ChangeFontText2 (Variables|Default|GetWBP_IconText%20Reference) (select (Utilities|IsValid (.FontObject (Utilities|Struct|BreakSlateFontInfo _font_2))) _font_2 (Variables|Default|GetDefaultFont))))
    (:then_4
      ;[1 1 1] Gets "Text" from macro and sends it to WBP_IconText
      (Default|ChangeText (Variables|Default|GetWBP_IconText%20Reference) (Variables|Default|GetText))
      (Default|ChangeText2 (Variables|Default|GetWBP_IconText%20Reference) (Variables|Default|GetText2)))
    (:then_5
      ;[1 1 1] Scale By Distance -  if distance is under scale minimum distance value then it doesn't scale. If the distance is bigger it starts scaling from there. If 'Scale Minimum Distance' is equal to 1000, then when distance to widget equals 2000 the scale is half: 1000/2000.
      (if (Variables|Default|GetScaleByDistance)
        (if (<= _returnvalue_4 _scaleminimumdistance)
          (Widget|Transform|SetRenderScale (Variables|Default|GetWBP_IconText%20Reference) "(X=1.000000,Y=1.000000)")
          (else
            (Widget|Transform|SetRenderScale (Variables|Default|GetWBP_IconText%20Reference) (Math|Vector2D|MakeVector2D _returnvalue_5 _returnvalue_5))))))
    (:then_6
      ;[1 1 1] Override Height and Width of Icon. Default is 32 by 32.
      (Default|SetHeightandWidthOfIcon (Variables|Default|GetWBP_IconText%20Reference) (Variables|Default|GetHeight%20Size) (Variables|Default|GetWidth%20Size)))
    (:then_7
      ;[1 1 1] Self Destroys After Time On Screen value in seconds
      (Default|SetTextDamageTimeonScreen (Variables|Default|GetWBP_IconText%20Reference) _timeonscreen)
      (Default|WidgetPlayAnimation (Variables|Default|GetWBP_IconText%20Reference) (Variables|Default|GetAnimationType))
      (Utilities|FlowControl|Delay _timeonscreen)
      (Actor|DestroyActor))))

(fn ConstructionScript)