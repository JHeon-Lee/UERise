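; BP_NPC002 is a village quest NPC that the player controller possesses to open quest acceptance.
; Its sphere detects the player through BPI_IsPlayer, toggles a prompt widget (turned toward the camera once at BeginPlay), registers as nearby NPC and caches the RealUtusi character.
; Possession sets up quest UI with UI-only input; IA_B fades, re-possesses the character and restores village mode.
; The construction script makes body, hair and face meshes follow the main mesh's pose.
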(event OnComponentBeginOverlap(Sphere)
  (params (OverlappedComponent :type Primitive%20Component%20Object%20Reference) (OtherActor :type Actor%20Object%20Reference) (OtherComp :type Primitive%20Component%20Object%20Reference) (OtherBodyIndex :type Integer) (bFromSweep :type Boolean) (SweepResult :type Hit%20Result%20Structure%20%28by%20ref%29))
  (bind _asbpi_is_player (Utilities|Casting|CastToBPI_IsPlayer OtherActor))
  (bind _bool (Default|IsPlayer _asbpi_is_player))
  (if _bool
    (Utilities|FlowControl|Sequence
      (:then_0
        (Rendering|SetVisibility (Variables|Default|GetWidget) true false)
        (Default|SetNearNPC _asbpi_is_player self))
      (:then_1
        (bind _asreal_utusi (Utilities|Casting|CastToRealUtusi OtherActor))
        (Variables|Default|SetPlayerCharacter _asreal_utusi)))))

(event OnComponentEndOverlap(Sphere)
  (params (OverlappedComponent :type Primitive%20Component%20Object%20Reference) (OtherActor :type Actor%20Object%20Reference) (OtherComp :type Primitive%20Component%20Object%20Reference) (OtherBodyIndex :type Integer))
  (bind _asbpi_is_player (Utilities|Casting|CastToBPI_IsPlayer OtherActor))
  (bind _bool (Default|IsPlayer _asbpi_is_player))
  (if _bool
    (Utilities|FlowControl|Sequence
      (:then_0
        (Rendering|SetVisibility (Variables|Default|GetWidget) false false)
        (Default|SetNearNPC _asbpi_is_player))
      (:then_1
        (Variables|Default|SetPlayerCharacter 0)))))

(event Input|EnhancedActionEvents|EnhancedInputActionIA_B
  (params (ActionValue :type Boolean) (ElapsedSeconds :type Float%20%28double-precision%29) (TriggeredSeconds :type Float%20%28double-precision%29) (InputAction :type Input%20Action%20Object%20Reference :default "/Game/InputSystem/IA_B.IA_B"))
  (bind _returnvalue (Game|GetPlayerController 0))
  (:Started
    (CameraFades|StartCameraFade :self (Game|GetPlayerCameraManager 0) :FromAlpha 1.0 :Duration 0.8)
    (Pawn|Possess _returnvalue (Variables|Default|GetPlayerCharacter))
    (bind _asbp_mhplayer_controller (Utilities|Casting|CastToBP_MHPlayerController _returnvalue))
    (Default|ChangeVillageMode _asbp_mhplayer_controller)))

(event EventBeginPlay
  (bind _widget (Variables|Default|GetWidget))
  (Transformation|SetWorldRotation _widget (Math|Rotator|FindLookatRotation (Transformation|GetWorldLocation _widget) (Transformation|GetWorldLocation (Variables|/Script/Engine.PlayerCameraManager|GetTransformComponent (Game|GetPlayerCameraManager 0)))) false false))

(event EventPossessed
  (params (NewController :type Controller%20Object%20Reference))
  (bind _returnvalue (Game|GetPlayerController 0))
  (Rendering|SetVisibility (Variables|Default|GetWidget) false false)
  (bind _asbp_mhplayer_controller (Utilities|Casting|CastToBP_MHPlayerController NewController))
  (Default|AddQuestAcceptance _asbp_mhplayer_controller)
  (Default|SetQuestEnum _asbp_mhplayer_controller "NewEnumerator2")
  (Variables|/Script/Engine.PlayerController|SetbShowMouseCursor _returnvalue true)
  (Input|SetInputModeUIOnly _returnvalue 0 "DoNotLock" false))

(fn ConstructionScript
  (Components|SkinnedMesh|SetLeaderPoseComponent (Variables|Default|Getnpc002_00_body_meshout) (Variables|Character|GetMesh) false false))