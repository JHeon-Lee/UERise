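; BP_Otomo is the rideable dog companion of the RealUtusi player, switching between follow, ready-to-ride, ride and hide modes.
; AIFollow drives following, while a dig montage and random reachable point support warping when pathing fails or distance grows.
; Ready-to-ride turns the dog and can start riding up close.
; Riding possesses the dog, pins the player to spine sockets and steers relative to the player's camera until IA_A dismounts.
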(event Custom|WarpToPlayer
  (Transformation|SetActorLocation (Variables|Default|GetWarpPoint) false false))

(event Input|EnhancedActionEvents|EnhancedInputActionIA_A
  (params (ActionValue :type Boolean) (ElapsedSeconds :type Float%20%28double-precision%29) (TriggeredSeconds :type Float%20%28double-precision%29) (InputAction :type Input%20Action%20Object%20Reference :default "/Game/InputSystem/IA_A.IA_A"))
  (:Started
    (CallFunction|GiveControltoPlayer)
    (CallFunction|SwitchMode "NewEnumerator0")))

(event EventBeginPlay
  (bind _aifollow (Variables|Default|GetAIFollow))
  (bind _asreal_utusi (Utilities|Casting|CastToRealUtusi (Game|GetPlayerCharacter 0)))
  (Variables|Default|SetReal%20Utusi _asreal_utusi)
  (Variables|/Game/Characters/CharacterComponent/MH_AIFollow.MH_AIFollow_C|SetPathEndOffset _aifollow "(X=100.000000,Y=0.000000)")
  (Variables|/Game/Characters/CharacterComponent/MH_AIFollow.MH_AIFollow_C|SetNearLimitToUtusi _aifollow 4e+02))

(event Collision|EventActorBeginOverlap
  (params (OtherActor :type Actor%20Object%20Reference)))

(event EventTick
  (params (DeltaSeconds :type Float%20%28single-precision%29))
  (Utilities|Array|SetArrayElem (Variables|Default|GetBoolArray) 1 (AI|Components|NavMovement|IsMovingonGround (Variables|Character|GetCharacterMovement)))
  (CallFunction|TooFarWarp)
  (switch Utilities|FlowControl|Switch|SwitchonOtomoMode (Variables|Default|GetOtomoMode)
    (:NewEnumerator0
      (CallFunction|Follow))
    (:NewEnumerator1
      (CallFunction|RideTick))
    (:NewEnumerator2
      (CallFunction|ReadyRideTick))
    (:NewEnumerator3
      (Components|Tick|SetComponentTickEnabled (Variables|Default|GetAIFollow) false))))

(fn ConstructionScript
  (Components|SkinnedMesh|SetLeaderPoseComponent (Variables|Default|GetSkeletalMesh1) (Variables|Character|GetMesh) false false))

(fn UtusiCamRotate
  (params (InVec :type Vector%202D%20Structure))
  (bind (_x _y) (Math|Vector2D|BreakVector2D InVec))
  (bind _real_utusi (Variables|Default|GetReal%20Utusi))
  (bind _cameraboom (Variables|/Script/UERise.MH_PlayerCharacter|GetCameraBoom _real_utusi))
  (bind _relativerotation (Variables|/Script/Engine.SceneComponent|GetRelativeRotation _cameraboom))
  (Transformation|AddRelativeRotation _cameraboom (Math|Rotator|MakeRotator 0.0 (* _y -1.0) _x) false false)
  (Transformation|SetRelativeRotation _cameraboom (Math|Rotator|MakeRotator 0.0 (Math|Float|Clamp(Float) (.pitch _relativerotation) -7e+01 7e+01) (.yaw _relativerotation)) false false))

(fn DogRotate
  (bind _returnvalue (Utilities|Time|GetWorldDeltaSeconds))
  (bind _actionvalue (Variables|Default|GetActionValue))
  (if (not (Utilities|Operators|EqualEqual :A (Variables|Default|GetActionValue) :ErrorTolerance 0.01))
    (Transformation|SetActorRotation (Math|Rotator|MakeRotator 0.0 0.0 (.yaw (Class|KismetMathLibrary|RInterptoConstant (Math|Rotator|MakeRotator 0.0 0.0 (.yaw (Transformation|GetActorRotation))) (Math|Rotator|MakeRotator 0.0 0.0 (+ (.yaw (.rotation (Transformation|GetRelativeTransform (Variables|/Script/UERise.MH_PlayerCharacter|GetCameraBoom (Variables|Default|GetReal%20Utusi))))) (.yaw (Math|Conversions|RotationFromXVector (Math|Vector|MakeVector (.x _actionvalue) (* (.y _actionvalue) -1.0) 0.0))))) _returnvalue (/ (Variables|Default|GetRotateSpeed) _returnvalue)))))))

(fn RideTick
  (bind _returnvalue (Transformation|GetActorRotation))
  (Utilities|FlowControl|Sequence
    (:then_0
      (Variables|Default|SetPressWASD (not (Utilities|Operators|EqualEqual :A (Input|EnhancedActionValues|GetIA_Move))))
      (Variables|Default|SetPressRB (Input|EnhancedActionValues|GetIA_RB))
      (Variables|Default|SetActionValue (Input|EnhancedActionValues|GetIA_Move))
      (CallFunction|DogRotate)
      (Variables|Default|SetSpeed (Math|Float|Max(Float) (Math|Float|Absolute(Float) (.x (Variables|Default|GetActionValue))) (Math|Float|Absolute(Float) (.y (Variables|Default|GetActionValue)))))
      (CallFunction|UtusiCamRotate (Input|EnhancedActionValues|GetIA_Look))
      ;[1 1 1] Player 위치, 회전 조작
      (if (Utilities|Enum|Equal(Enum) (Variables|/Game/Characters/Utusi/Bluprints/RealUtusi.RealUtusi_C|GetWeaponState (Variables|Default|GetReal%20Utusi)) "NewEnumerator2")
        (if (!= (Animation|Montage|GetCurrentActiveMontage (Components|SkeletalMesh|GetAnimInstance (Variables|/Script/Engine.Character|GetMesh (Variables|Default|GetReal%20Utusi)))) "/Game/Characters/Utusi/Anim/Ride/plc_Ride_005_031_Montage.plc_Ride_005_031_Montage")
          (Transformation|SetActorLocationAndRotation (Variables|Default|GetReal%20Utusi) (+ (Transformation|GetSocketLocation (Variables|Character|GetMesh) "Spine_00") "0.000000,0.000000,100.000000") _returnvalue)
          (else
            (Transformation|SetActorLocationAndRotation (Variables|Default|GetReal%20Utusi) (- (Transformation|GetSocketLocation (Variables|Character|GetMesh) "Spine_03") "0.000000,0.000000,20.000000") _returnvalue)))
        (if (and (not (Class|AnimInstance|IsAnyMontagePlaying (Components|SkeletalMesh|GetAnimInstance (Variables|Character|GetMesh)))) (not (AI|Components|NavMovement|IsMovingonGround (Variables|Character|GetCharacterMovement))))
          (Animation|PlayAnimMontage "/Game/Characters/Otomo/Motion/Jump1.Jump1" 1.0 "None"))))))

(fn FollowTick
  (if (not (Class|ActorComponent|IsComponentTickEnabled (Variables|Default|GetAIFollow)))
    (Components|Tick|SetComponentTickEnabled (Variables|Default|GetAIFollow) true)))

(fn SwitchMode
  (params (WhichMode :type OtomoMode%20Enum :default "NewEnumerator0"))
  (bind _returnvalue (Game|GetPlayerController 0))
  (bind _real_utusi (Variables|Default|GetReal%20Utusi))
  (switch Utilities|FlowControl|Switch|SwitchonOtomoMode WhichMode
    (:NewEnumerator0
      (Variables|Default|SetOtomoMode "NewEnumerator0")
      (Components|Tick|SetComponentTickEnabled (Variables|Default|GetAIFollow) true)
      (Variables|/Game/Characters/CharacterComponent/MH_AIFollow.MH_AIFollow_C|SetPathEndOffset (Variables|Default|GetAIFollow) "(X=100.000000,Y=0.000000)")
      (Variables|/Game/Characters/CharacterComponent/MH_AIFollow.MH_AIFollow_C|SetNearLimitToUtusi (Variables|Default|GetAIFollow) 4e+02))
    (:NewEnumerator1
      (Variables|Default|SetOtomoMode "NewEnumerator1")
      (Components|Tick|SetComponentTickEnabled (Variables|Default|GetAIFollow) false)
      (Pawn|Possess _returnvalue self)
      (Game|Player|SetViewTargetwithBlend _returnvalue (Variables|Default|GetReal%20Utusi) 0.0 "VTBlend_Linear" 0.0 false)
      (Variables|/Game/Characters/Utusi/Bluprints/RealUtusi.RealUtusi_C|SetWeaponState (Variables|Default|GetReal%20Utusi) "NewEnumerator2")
      (Pawn|Components|CharacterMovement|SetMovementMode (Variables|/Script/Engine.Character|GetCharacterMovement (Variables|Default|GetReal%20Utusi)) "MOVE_Flying" 0)
      (Variables|/Script/Engine.SpringArmComponent|SetTargetOffset (Variables|/Script/UERise.MH_PlayerCharacter|GetCameraBoom _real_utusi) (+ (* (Transformation|GetActorRightVector _real_utusi) -4e+01) "0.000000,0.000000,83.000000")))
    (:NewEnumerator2
      (Variables|Default|SetOtomoMode "NewEnumerator2")
      (Components|Tick|SetComponentTickEnabled (Variables|Default|GetAIFollow) false))))

(fn GiveControltoPlayer
  (Pawn|Possess (Game|GetPlayerController 0) (Variables|Default|GetReal%20Utusi))
  (Variables|/Game/Characters/Utusi/Bluprints/RealUtusi.RealUtusi_C|SetWeaponState (Variables|Default|GetReal%20Utusi) "NewEnumerator0")
  (Pawn|Components|CharacterMovement|SetMovementMode (Variables|/Script/Engine.Character|GetCharacterMovement (Variables|Default|GetReal%20Utusi)) "MOVE_Walking" 0)
  (Variables|/Script/Engine.SpringArmComponent|SetTargetOffset (Variables|/Script/UERise.MH_PlayerCharacter|GetCameraBoom (Variables|Default|GetReal%20Utusi)) "0.000000,0.000000,70.000000")
  (Animation|PlayAnimMontage (Variables|Default|GetReal%20Utusi) "/Game/Characters/Utusi/Anim/RealUnarmed/S_079_Montage.S_079_Montage" 1.0 "None"))

(fn GetAngleBtwTrgt
  (bind _returnvalue (Transformation|GetActorLocation))
  (bind _returnvalue_2 (Transformation|GetActorRightVector))
  (bind _real_utusi (Variables|Default|GetReal%20Utusi))
  (bind _returnvalue_3 (Transformation|GetActorLocation _real_utusi))
  (bind _returnvalue_4 (Transformation|GetActorForwardVector _real_utusi))
  (bind _returnvalue_5 (Transformation|GetActorForwardVector _real_utusi))
  (bind _returnvalue_6 (* _returnvalue_4 5e+01))
  (bind _returnvalue_7 (* _returnvalue_5 -5e+01))
  (bind _returnvalue_8 (+ _returnvalue_3 _returnvalue_6 _returnvalue_7))
  (bind _returnvalue_9 (Math|Rotator|FindLookatRotation _returnvalue _returnvalue_8))
  (bind _returnvalue_10 (Math|Vector|GetForwardVector _returnvalue_9))
  (Variables|Default|SetAngleBtwTrgt (- (Class|KismetMathLibrary|DegAtan2 (.x _returnvalue_2) (.y _returnvalue_2)) (Class|KismetMathLibrary|DegAtan2 (.x _returnvalue_10) (.y _returnvalue_10))))
  (Utilities|FlowControl|Sequence
    (:then_0
      (if (> (Variables|Default|GetAngleBtwTrgt) 1.8e+02)
        (Variables|Default|SetAngleBtwTrgt (- (Variables|Default|GetAngleBtwTrgt) 3.6e+02))))
    (:then_1
      (if (< (Variables|Default|GetAngleBtwTrgt) -1.8e+02)
        (bind _output_get (Variables|Default|SetAngleBtwTrgt (+ (Variables|Default|GetAngleBtwTrgt) 3.6e+02)))
        (return _output_get)))))

(fn ReadyRideTick
  (bind _real_utusi (Variables|Default|GetReal%20Utusi))
  (CallFunction|GetAngleBtwTrgt)
  (if (> (Math|Float|Absolute(Float) (Variables|Default|GetAngleBtwTrgt)) 3.0)
    (if (< (Variables|Default|GetAngleBtwTrgt) 0.0)
      (Class|Actor|AddActorWorldRotation (Math|Rotator|MakeRotator 0.0 0.0 (* (Variables|Default|GetReadyToRideRotSpeed) (Utilities|Time|GetWorldDeltaSeconds) -1.0)))
      (else
        (Class|Actor|AddActorWorldRotation (Math|Rotator|MakeRotator 0.0 0.0 (* (Variables|Default|GetReadyToRideRotSpeed) (Utilities|Time|GetWorldDeltaSeconds))))))
    (if (< (Math|Vector|Distance(Vector) (Transformation|GetActorLocation (Variables|Default|GetReal%20Utusi)) (Transformation|GetActorLocation)) 5e+01)
      (if (Math|Boolean|ORBoolean (Class|AnimInstance|IsAnyMontagePlaying (Components|SkeletalMesh|GetAnimInstance (Variables|/Script/Engine.Character|GetMesh _real_utusi))) (Utilities|Enum|NotEqual(Enum) (Variables|/Script/Engine.CharacterMovementComponent|GetMovementMode (Variables|/Script/Engine.Character|GetCharacterMovement _real_utusi)) "MOVE_Walking") (Utilities|Enum|Equal(Enum) (Variables|/Game/Characters/Utusi/Bluprints/RealUtusi.RealUtusi_C|GetWeaponState _real_utusi) "NewEnumerator1"))
        (CallFunction|SwitchMode "NewEnumerator0")
        (else
          (CallFunction|SwitchMode "NewEnumerator1")
          (Animation|PlayAnimMontage (Variables|Default|GetReal%20Utusi) "/Game/Characters/Utusi/Anim/Ride/plc_Ride_005_031_Montage.plc_Ride_005_031_Montage" 1.0 "None"))))))

(fn Follow
  (bind _real_utusi (Variables|Default|GetReal%20Utusi))
  (bind _returnvalue (Transformation|GetActorLocation _real_utusi))
  (bind (_randomlocation _returnvalue_2) (AI|Navigation|GetRandomReachablePointinRadius _returnvalue 3e+02 0 0))
  (if (not (Variables|/Game/Characters/CharacterComponent/MH_AIFollow.MH_AIFollow_C|GetCanFindPath (Variables|Default|GetAIFollow)))
    (if (AI|Components|NavMovement|IsMovingonGround (Pawn|GetMovementComponent (Variables|Default|GetReal%20Utusi)))
      (if _returnvalue_2
        (Variables|Default|SetWarpPoint (+ _randomlocation "0.000000,0.000000,80.000000"))
        (if (!= (Animation|Montage|GetCurrentActiveMontage (Components|SkeletalMesh|GetAnimInstance (Variables|Character|GetMesh))) "/Game/Characters/Otomo/Motion/digToPlayer.digToPlayer")
          (Animation|PlayAnimMontage "/Game/Characters/Otomo/Motion/digToPlayer.digToPlayer" 1.0 "None"))))))

(fn TooFarWarp
  (bind _real_utusi (Variables|Default|GetReal%20Utusi))
  (bind _returnvalue (Transformation|GetActorLocation _real_utusi))
  (bind (_randomlocation _returnvalue_2) (AI|Navigation|GetRandomReachablePointinRadius _returnvalue 3e+02 0 0))
  (if (> (Math|Vector|Distance(Vector) (Transformation|GetActorLocation (Variables|Default|GetReal%20Utusi)) (Transformation|GetActorLocation self)) 2e+03)
    (if _returnvalue_2
      (Variables|Default|SetWarpPoint (+ _randomlocation "0.000000,0.000000,80.000000"))
      (if (not (== (Animation|GetCurrentMontage :!class /Script/Engine.Character) "/Game/Characters/Otomo/Motion/digToPlayer.digToPlayer"))
        (Animation|PlayAnimMontage "/Game/Characters/Otomo/Motion/digToPlayer.digToPlayer" 1.0 "None")))))