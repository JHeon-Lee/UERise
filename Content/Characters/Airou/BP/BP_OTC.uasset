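; Airou companion character that follows the player (RealUtusi) and fights beside them.
; Tick switches between follow and fight modes, playing a dig-in montage to warp when the player is too far or unreachable.
; FindEnemy pauses AIFollow and picks a random attack and position; FightTick rotates toward it and plays that attack's montage within range.
; Separate events handle projectile spawning, sphere-trace weapon hits with damage text, teleporting, and returning to follow.
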(event Custom|FindEnemy
  (params (enemy :type Actor%20Object%20Reference))
  (if (Utilities|Enum|Equal(Enum) (Variables|Default|GetOtcMode) "NewEnumerator0")
    (Variables|Default|SetOtcMode "NewEnumerator1")
    (Variables|Default|SetEnemyActor enemy)
    (Components|Tick|SetComponentTickEnabled (Variables|Default|GetAIFollow) false)
    (CallFunction|SelectNextAtkPattern)))

(event Custom|BattleOver
  (if (Class|AnimInstance|IsAnyMontagePlaying (Components|SkeletalMesh|GetAnimInstance (Variables|Character|GetMesh))) :!label _label
    (Utilities|FlowControl|Delay 0.5)
    (goto _label)
    (else
      (Variables|Default|SetOtcMode "NewEnumerator0")
      (Components|Tick|SetComponentTickEnabled (Variables|Default|GetAIFollow) true))))

(event Custom|SpawnProjectil
  (bind _returnvalue (Transformation|GetActorTransform))
  (Game|SpawnActorfromClass (Utilities|Select :Index (Variables|Default|GetAttackPattern) :NewEnumerator1 0 :NewEnumerator2 "/Game/Characters/Airou/Model/ItemProjectile/projectileBomb.projectileBomb_C" :NewEnumerator3 "/Game/Characters/Airou/Model/ItemProjectile/projectileGiant.projectileGiant_C" :NewEnumerator4 "/Game/Characters/Airou/Model/ItemProjectile/projectileBone.projectileBone_C") (Math|Transform|MakeTransform (.location _returnvalue) (Math|Conversions|RotationFromXVector (Transformation|GetActorRightVector)) (.scale _returnvalue)) "Undefined" 0 0))

(event Custom|AtkCheck
  (bind _returnvalue (Math|Random|RandomIntegerinRange 12 20))
  (bind _mesh (Variables|Character|GetMesh))
  (bind _returnvalue_2 (Math|Conversions|ToFloat(Integer) _returnvalue))
  (bind (_outhit _returnvalue_3) (Collision|SphereTraceForObjects (Transformation|GetSocketLocation _mesh "RWeapon") (Transformation|GetSocketLocation _mesh "RWeaponEnd") 3e+01 (Utilities|Array|MakeArray "ObjectTypeQuery4") false 0 "None"))
  (if _returnvalue_3
    (Niagara|SpawnSystematLocation "/Game/MarketContent/SlashHitAndStabHit/Particles/Niagara/NS_ky_stabHit12.NS_ky_stabHit12" (.Location (Collision|BreakHitResult _outhit)))
    (Game|Damage|ApplyDamage (.HitActor (Collision|BreakHitResult _outhit)) _returnvalue_2 0 0)
    (Utilities|SpawnDynamicTextatWorld :Spawn%20Transform%20Location (.Location (Collision|BreakHitResult _outhit)) :Text%20Damage (Utilities|Text|ToText(Float) _returnvalue_2 "HalfToEven") :Font (Variables|Default|GetFont) :Font%20Color "(R=0.250000,G=0.250000,B=0.250000,A=1.000000)")))

(event Custom|WarpToPlayer
  (bind _real_utusi (Variables|Default|GetReal%20Utusi))
  (bind _returnvalue (Transformation|GetActorLocation _real_utusi))
  (bind (_randomlocation _returnvalue_2) (AI|Navigation|GetRandomReachablePointinRadius _returnvalue 3e+02 0 0))
  (if _returnvalue_2
    (Transformation|SetActorLocation (+ _randomlocation "0.000000,0.000000,80.000000") false false)))

(event EventBeginPlay
  (bind _asreal_utusi (Utilities|Casting|CastToRealUtusi (Game|GetPlayerCharacter 0)))
  (Utilities|IsValid _asreal_utusi
    (:Is%20Valid
      (Variables|Default|SetReal%20Utusi _asreal_utusi))
    (:Is%20Not%20Valid
      (Development|PrintString "RealUtusi Not valid"))))

(event Collision|EventActorBeginOverlap
  (params (OtherActor :type Actor%20Object%20Reference)))

(event EventTick
  (params (DeltaSeconds :type Float%20%28single-precision%29))
  (CallFunction|ToofarWarp)
  (switch Utilities|FlowControl|Switch|SwitchonotcMode (Variables|Default|GetOtcMode)
    (:NewEnumerator0
      (CallFunction|FollowTick))
    (:NewEnumerator1
      (CallFunction|FightTick))))

(fn ConstructionScript
  (Components|SkinnedMesh|SetLeaderPoseComponent (Variables|Default|Getota_helm007) (Variables|Character|GetMesh) false false))

(fn SelectNextAtkPattern
  (bind _enemyactor (Variables|Default|GetEnemyActor))
  (bind _returnvalue (Transformation|GetActorLocation _enemyactor))
  (Variables|Default|SetAttackPattern (Utilities|Enum|ByteToEnumotcAtkPattern (Math|Conversions|ToByte(Integer) (Math|Random|RandomIntegerinRange 0 3))))
  (Utilities|IsValid _enemyactor
    (:Is%20Valid
      (bind _outhit (Collision|LineTraceForObjects (+ _returnvalue (* (Transformation|GetActorForwardVector (Variables|Default|GetReal%20Utusi)) -1e+03)) _returnvalue (Utilities|Array|MakeArray "ObjectTypeQuery4") false 0 "None"))
      (if (.bBlockingHit (Collision|BreakHitResult _outhit))
        (bind _output_get (Variables|Default|SetAtkPosition (+ (.Location (Collision|BreakHitResult _outhit)) (* (Transformation|GetActorForwardVector (Variables|Default|GetReal%20Utusi)) (Utilities|Select :Index (Variables|Default|GetAttackPattern) :NewEnumerator1 1e+02 :NewEnumerator2 5e+02 :NewEnumerator3 6e+02 :NewEnumerator4 4e+02) -1.0))))
        (else
          (Variables|Default|SetAtkPosition (* (Utilities|Select :Index (Variables|Default|GetAttackPattern) :NewEnumerator1 1e+02 :NewEnumerator2 5e+02 :NewEnumerator3 6e+02 :NewEnumerator4 4e+02) -1.0 (Transformation|GetActorRightVector (Variables|Default|GetEnemyActor)))))))))

(fn JumpAtk)

(fn GetAngletoTrgtLocation
  (params (TrgtLocation :type Vector))
  (bind _returnvalue (Transformation|GetActorLocation))
  (bind _returnvalue_2 (Transformation|GetActorRightVector))
  (bind _returnvalue_3 (Math|Rotator|FindLookatRotation _returnvalue TrgtLocation))
  (bind _returnvalue_4 (Math|Vector|GetForwardVector _returnvalue_3))
  (Variables|Default|SetAngleBtwTrgt (- (Class|KismetMathLibrary|DegAtan2 (.x _returnvalue_2) (.y _returnvalue_2)) (Class|KismetMathLibrary|DegAtan2 (.x _returnvalue_4) (.y _returnvalue_4))))
  (Utilities|FlowControl|Sequence
    (:then_0
      (if (> (Variables|Default|GetAngleBtwTrgt) 1.8e+02)
        (Variables|Default|SetAngleBtwTrgt (- (Variables|Default|GetAngleBtwTrgt) 3.6e+02))))
    (:then_1
      (if (< (Variables|Default|GetAngleBtwTrgt) -1.8e+02)
        (Variables|Default|SetAngleBtwTrgt (+ (Variables|Default|GetAngleBtwTrgt) 3.6e+02))))))

(fn RotatetoTrgtLocation
  (if (> (Math|Float|Absolute(Float) (Variables|Default|GetAngleBtwTrgt)) 3.0)
    (if (< (Variables|Default|GetAngleBtwTrgt) 0.0)
      (Class|Actor|AddActorWorldRotation (Math|Rotator|MakeRotator 0.0 0.0 (* (Variables|Default|GetRotateSpeed) (Utilities|Time|GetWorldDeltaSeconds) -1.0)))
      (else
        (Class|Actor|AddActorWorldRotation (Math|Rotator|MakeRotator 0.0 0.0 (* (Variables|Default|GetRotateSpeed) (Utilities|Time|GetWorldDeltaSeconds))))))))

(fn FightTick
  (bind _returnvalue (Transformation|GetActorLocation))
  (bind _atkposition (Variables|Default|GetAtkPosition))
  (if (not (Class|AnimInstance|IsAnyMontagePlaying (Components|SkeletalMesh|GetAnimInstance (Variables|Character|GetMesh))))
    (if (not (Math|Vector|VectorIsZero (Variables|Default|GetAtkPosition)))
      (CallFunction|GetAngletoTrgtLocation (Variables|Default|GetAtkPosition))
      (CallFunction|RotatetoTrgtLocation)
      (if (< (Math|Vector|Distance(Vector) (Math|Vector|MakeVector (.x _atkposition) (.y _atkposition) 0.0) (Math|Vector|MakeVector (.x _returnvalue) (.y _returnvalue) 0.0)) (Variables|Default|GetAcceptanceRadius))
        (CallFunction|GetAngletoTrgtLocation (Transformation|GetActorLocation (Variables|Default|GetEnemyActor)))
        (Class|Actor|AddActorWorldRotation (Math|Rotator|MakeRotator 0.0 0.0 (Variables|Default|GetAngleBtwTrgt)))
        (Animation|PlayAnimMontage (Utilities|Select :Index (Variables|Default|GetAttackPattern) :NewEnumerator1 "/Game/Characters/Airou/Motion/02/airou_00_02005_Montage.airou_00_02005_Montage" :NewEnumerator2 "/Game/Characters/Airou/Motion/02/airou_00_02029_Montage.airou_00_02029_Montage" :NewEnumerator3 "/Game/Characters/Airou/Motion/02/airou_00_02062_Montage.airou_00_02062_Montage" :NewEnumerator4 "/Game/Characters/Airou/Motion/02/airou_00_02056_Montage.airou_00_02056_Montage") 1.0 "None")))))

(fn FollowTick
  (bind _real_utusi (Variables|Default|GetReal%20Utusi))
  (bind _returnvalue (Transformation|GetActorLocation _real_utusi))
  (bind (_randomlocation _returnvalue_2) (AI|Navigation|GetRandomReachablePointinRadius _returnvalue 3e+02 0 0))
  (if (not (Variables|/Game/Characters/CharacterComponent/MH_AIFollow.MH_AIFollow_C|GetCanFindPath (Variables|Default|GetAIFollow)))
    (if (AI|Components|NavMovement|IsMovingonGround (Pawn|GetMovementComponent (Variables|Default|GetReal%20Utusi)))
      (if _returnvalue_2
        (Variables|Default|SetWarpPoint (+ _randomlocation "0.000000,0.000000,80.000000"))
        (if (not (== (Animation|Montage|GetCurrentActiveMontage (Components|SkeletalMesh|GetAnimInstance (Variables|Character|GetMesh))) "/Game/Characters/Airou/Motion/04/otc_digin_Montage.otc_digin_Montage"))
          (Animation|PlayAnimMontage "/Game/Characters/Airou/Motion/04/otc_digin_Montage.otc_digin_Montage" 1.0 "None"))))))

(fn ToofarWarp
  (bind _real_utusi (Variables|Default|GetReal%20Utusi))
  (bind _returnvalue (Transformation|GetActorLocation _real_utusi))
  (bind (_randomlocation _returnvalue_2) (AI|Navigation|GetRandomReachablePointinRadius _returnvalue 3e+02 0 0))
  (if (> (Math|Vector|Distance(Vector) (Transformation|GetActorLocation (Variables|Default|GetReal%20Utusi)) (Transformation|GetActorLocation self)) 2e+03)
    (if _returnvalue_2
      (Variables|Default|SetWarpPoint (+ _randomlocation "0.000000,0.000000,80.000000"))
      (if (not (== (Animation|GetCurrentMontage :!class /Script/Engine.Character) "/Game/Characters/Airou/Motion/04/otc_digin_Montage.otc_digin_Montage"))
        (Animation|PlayAnimMontage "/Game/Characters/Airou/Motion/04/otc_digin_Montage.otc_digin_Montage" 1.0 "None")))))