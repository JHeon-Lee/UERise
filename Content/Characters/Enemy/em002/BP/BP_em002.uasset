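; BP_em002 is an enemy character Blueprint that reacts to point damage with floating damage numbers and a montage.
; The bone closest to the hit is matched against PartInfo, whose hardness value scales the displayed damage as a percentage.
; Text font and color distinguish critical, effective and weak hits, with critical styling requiring a CriticalDamageType and sufficient hardness.
; Scaled damage above a threshold plays a montage; leftover pathfinding nodes never run.
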(event EventBeginPlay)

(event Collision|EventActorBeginOverlap
  (params (OtherActor :type Actor%20Object%20Reference)))

(event EventTick
  (params (DeltaSeconds :type Float%20%28single-precision%29)))

(event Game|Damage|EventPointDamage
  (params (Damage :type Float%20%28single-precision%29) (DamageType :type Damage%20Type%20Object%20Reference) (HitLocation :type Vector :default "0, 0, 0") (HitNormal :type Vector :default "0, 0, 0") (HitComponent :type Primitive%20Component%20Object%20Reference) (BoneName :type Name :default "None") (ShotFromDirection :type Vector :default "0, 0, 0") (InstigatedBy :type Controller%20Object%20Reference) (DamageCauser :type Actor%20Object%20Reference) (HitInfo :type Hit%20Result%20Structure%20%28by%20ref%29))
  (bind _location (Collision|BreakHitResult HitInfo))
  (Utilities|Casting|CastToCriticalDamageType DamageType
    (:then
      (Variables|Default|SetCritical true))
    (:CastFailed
      (Variables|Default|SetCritical false)))
  (for _array_element (Variables|Default|GetPartInfo)
    (if (Utilities|String|Contains (Utilities|String|ToString(Name) (.ReturnValue (Class|SkinnedMeshComponent|FindClosestBoneK2 (Variables|Character|GetMesh) _location 0.0))) (.bonename _array_element))
      (if (>= (.hardness _array_element) 45.0)
        (if (Variables|Default|GetCritical)
          (Utilities|SpawnDynamicTextatWorld :Spawn%20Transform%20Location _location :Animation "NewEnumerator3" :Text%20Damage (Utilities|Text|ToText(Float) (Math|Conversions|ToFloat(Integer) (Math|Float|Round (* Damage (.hardness _array_element) 0.01))) "HalfToEven") :Font (Variables|Default|GetCritFont) :Font%20Color "(R=1.000000,G=0.298944,B=0.047060,A=1.000000)" :Font%202%20Color "(R=1.000000,G=0.071004,B=0.041157,A=1.000000)")
          (else
            (Utilities|SpawnDynamicTextatWorld :Spawn%20Transform%20Location _location :Animation "NewEnumerator3" :Text%20Damage (Utilities|Text|ToText(Float) (Math|Conversions|ToFloat(Integer) (Math|Float|Round (* Damage (.hardness _array_element) 0.01))) "HalfToEven") :Font (Variables|Default|GetEffectiveDmg) :Font%20Color "(R=1.000000,G=0.592295,B=0.000000,A=1.000000)")))
        (else
          (Utilities|SpawnDynamicTextatWorld :Spawn%20Transform%20Location _location :Animation "NewEnumerator3" :Text%20Damage (Utilities|Text|ToText(Float) (Math|Conversions|ToFloat(Integer) (Math|Float|Round (* Damage (.hardness _array_element) 0.01))) "HalfToEven") :Font (Variables|Default|GetNotEffectiveDmg) :Font%20Color "(R=0.661458,G=0.661458,B=0.661458,A=1.000000)" :Font%202%20Color "(R=1.000000,G=0.071004,B=0.041157,A=1.000000)")))
      (if (> (Math|Conversions|ToFloat(Integer) (Math|Float|Round (* Damage (.hardness _array_element) 0.01))) 5e+02)
        (Animation|PlayAnimMontage "/Game/Characters/Enemy/em002/Motion/03/em002_00_03008_Montage.em002_00_03008_Montage" 1.0 "None")))))

(fn ConstructionScript)