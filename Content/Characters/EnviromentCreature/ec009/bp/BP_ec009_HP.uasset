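; Environment creature pickup (ec009 HP variant) that grants a player-controlled RealUtusi a max HP bonus on overlap.
; On overlap it requires a valid inventory, then adds a fixed step to the character's MaxHpModifier, clamped to a cap.
; It then tints and restarts the character's StatBirdEft effect and adds itself to the inventory through AGRItem PickUpItem.
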(event EventBeginPlay)

(event Collision|EventActorBeginOverlap
  (params (OtherActor :type Actor%20Object%20Reference))
  (bind _asreal_utusi (Utilities|Casting|CastToRealUtusi OtherActor))
  (if (Pawn|IsPlayerControlled _asreal_utusi)
    (Utilities|IsValid (Class|AGRLibrary|GetInventory _asreal_utusi)
      (:Is%20Valid
        (Variables|/Script/UERise.MH_PlayerCharacter|SetMaxHpModifier _asreal_utusi (Math|Float|Clamp(Float) (+ (Variables|/Script/UERise.MH_PlayerCharacter|GetMaxHpModifier _asreal_utusi) 5.0) 0.0 5e+01))
        (Effects|Components|ParticleSystem|SetColorParameter (Variables|/Game/Characters/Utusi/Bluprints/RealUtusi.RealUtusi_C|GetStatBirdEft _asreal_utusi) "Color" "(R=1.717476,G=30.000000,B=0.000000,A=1.000000)")
        (Components|Activation|SetActive (Variables|/Game/Characters/Utusi/Bluprints/RealUtusi.RealUtusi_C|GetStatBirdEft _asreal_utusi) true true)
        (Class|AGRItemComponent|PickUpItem (Variables|Default|GetAGR_Item) (Class|AGRLibrary|GetInventory _asreal_utusi)))
      (:Is%20Not%20Valid
        (Development|PrintString "inventory not valid")))))

(fn ConstructionScript)