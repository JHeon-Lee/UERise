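; BP_ky_stab is an actor that repeatedly plays a stab motion with a visual effect, with optional mesh visibility.
; A timeline drives the Pivot along X, and delays chained from its update activate either Niagara or Cascade particles, chosen by UseNiagara.
; After a further delay both systems deactivate and the timeline restarts, forming a continuous loop.
; The construction script offsets both effect components along X by FxOfsX.
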(event EventBeginPlay
  ;[1 1 1] init
  (Rendering|SetVisibility (Variables|Default|GetStaticMesh) (Variables|Default|GetisMeshVisible) false)
  (Components|Activation|Deactivate (Variables|Default|GetParticleSystem))
  ;[1 1 1] fx control
  (bind _xvalue (Timeline|Timeline_0 PlayFromStart)
    (:Update
      (Transformation|SetRelativeLocation (Variables|Default|GetPivot) (Math|Vector|MakeVector _xvalue 0.0 0.0) false false)
      (Utilities|FlowControl|Delay 0.15)
      (if (Variables|Default|GetuseNiagara)
        (Components|Activation|Activate (Variables|Default|GetNiagara) false)
        (else
          (Components|Activation|Activate (Variables|Default|GetParticleSystem) false)))
      (Utilities|FlowControl|Delay 1.0)
      (Components|Activation|Deactivate (Variables|Default|GetParticleSystem))
      (Timeline|Timeline_0 PlayFromStart))))

(event Collision|EventActorBeginOverlap
  (params (OtherActor :type Actor%20Object%20Reference)))

(event EventTick
  (params (DeltaSeconds :type Float%20%28single-precision%29)))

(fn ConstructionScript
  ;[1 1 1] fx offset
  (Transformation|SetRelativeLocation (Variables|Default|GetParticleSystem) (Math|Vector|MakeVector (Variables|Default|GetFxOfsX) 0.0 0.0) false false))