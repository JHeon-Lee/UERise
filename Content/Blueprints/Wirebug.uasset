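; Wirebug is a collectible actor that raises the player's maximum wirebug count when it takes damage.
; Its overlap sphere shows a prompt widget, rotated toward the camera once at BeginPlay, and registers the actor with RealUtusi as a nearby "벌꿀" (honey) prop.
; AnyDamage plays a timeline that marks it picked, hides the widget and fades mesh opacity, then credits the damage causer through BPI_IsPlayer with a pickup sound.
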(event OnComponentBeginOverlap(Sphere)
  (params (OverlappedComponent :type Primitive%20Component%20Object%20Reference) (OtherActor :type Actor%20Object%20Reference) (OtherComp :type Primitive%20Component%20Object%20Reference) (OtherBodyIndex :type Integer) (bFromSweep :type Boolean) (SweepResult :type Hit%20Result%20Structure%20%28by%20ref%29))
  (Utilities|FlowControl|Sequence
    (:then_0
      (bind _asbpi_is_player (Utilities|Casting|CastToBPI_IsPlayer OtherActor))
      (bind _bool (Default|IsPlayer _asbpi_is_player))
      (if (and _bool (not (Variables|Default|GetPicked)))
        (Rendering|SetVisibility (Variables|Default|GetWidget) true false)
        (Audio|PlaySound2D "/Game/ImportSource/Sound/UI/ui100/UIClose.UIClose" 1.0 1.0 0.0 0 0)))
    (:then_1
      (bind _asreal_utusi (Utilities|Casting|CastToRealUtusi OtherActor))
      (if (and (Pawn|IsPlayerControlled _asreal_utusi) (Utilities|IsValid _asreal_utusi))
        (Default|SetNearProp _asreal_utusi self "벌꿀")))))

(event OnComponentEndOverlap(Sphere)
  (params (OverlappedComponent :type Primitive%20Component%20Object%20Reference) (OtherActor :type Actor%20Object%20Reference) (OtherComp :type Primitive%20Component%20Object%20Reference) (OtherBodyIndex :type Integer))
  (bind _asbpi_is_player (Utilities|Casting|CastToBPI_IsPlayer OtherActor))
  (bind _bool (Default|IsPlayer _asbpi_is_player))
  (if _bool
    (Default|SetNearProp (stale OnComponentBeginOverlap(Sphere) _asreal_utusi) 0 "")
    (Rendering|SetVisibility (Variables|Default|GetWidget) false false)))

(event EventBeginPlay
  (bind _widget (Variables|Default|GetWidget))
  (Transformation|SetWorldRotation _widget (Math|Rotator|FindLookatRotation (Transformation|GetWorldLocation _widget) (Transformation|GetWorldLocation (Variables|/Script/Engine.PlayerCameraManager|GetTransformComponent (Game|GetPlayerCameraManager 0)))) false false))

(event Game|Damage|EventAnyDamage
  (params (Damage :type Float%20%28single-precision%29) (DamageType :type Damage%20Type%20Object%20Reference) (InstigatedBy :type Controller%20Object%20Reference) (DamageCauser :type Actor%20Object%20Reference))
  (bind _timer (Timeline|Timeline Play)
    (:Update
      (Rendering|Material|SetScalarParameterValueonMaterials (Variables|Default|GetSkeletalMesh) "Opacity" _timer)
      (Variables|Default|SetPicked true)
      (Rendering|SetVisibility (Variables|Default|GetWidget) false false))
    (:Finished
      (bind _asbpi_is_player (Utilities|Casting|CastToBPI_IsPlayer DamageCauser))
      (Default|IncreaseMaxWirebugCount _asbpi_is_player)
      (Audio|PlaySound2D "/Game/ImportSource/Sound/플레이어/wirebugget.wirebugget" 1.0 1.0 0.0 0 0))))

(fn ConstructionScript)