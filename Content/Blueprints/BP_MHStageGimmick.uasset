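; BP_MHStageGimmick is a one-shot trigger that introduces the Rathalos monster when the player enters its volume.
; On overlap by an actor implementing BPI_IsPlayer, it lights the Rathalos icon on the HUD, plays a Level Sequence and switches the player controller to quest mode.
; After a fixed delay, it spawns the Rathalos character at a hardcoded location and switches the controller to field mode.
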(event OnComponentBeginOverlap(StageTrigger)
  (params (OverlappedComponent :type Primitive%20Component%20Object%20Reference) (OtherActor :type Actor%20Object%20Reference) (OtherComp :type Primitive%20Component%20Object%20Reference) (OtherBodyIndex :type Integer) (bFromSweep :type Boolean) (SweepResult :type Hit%20Result%20Structure%20%28by%20ref%29))
  (if (and (not (Variables|Default|GetIsTriggered)) (Utilities|DoesObjectImplementInterface OtherActor "/Game/Blueprints/BPI_IsPlayer.BPI_IsPlayer_C"))
    (Variables|Default|SetIsTriggered true)
    (bind _asmhplayer_controller (Utilities|Casting|CastToMHPlayerController (Game|GetPlayerController 0)))
    (bind _aswbp_mhhud (Utilities|Casting|CastToWBP_MHHUD (Variables|/Script/UERise.MHPlayerController|GetMHHUDWidget _asmhplayer_controller)))
    (Class|Image|SetOpacity (Variables|/Game/Characters/Utusi/UI/WBP_MonsterIcon.WBP_MonsterIcon_C|GetRathalosIcon (Variables|/Game/Characters/Utusi/UI/WBP_MHHUD.WBP_MHHUD_C|GetWBP_MonsterIcon _aswbp_mhhud)) 1.0)
    (bind (_outactor _returnvalue) (Sequencer|Player|CreateLevelSequencePlayer "/Game/Cinematics/Sequences/Sequence/SequenceMaster.SequenceMaster"))
    (Sequencer|Player|Play (Variables|/Script/LevelSequence.LevelSequenceActor|GetSequencePlayer _outactor) :!class /Script/MovieScene.MovieSceneSequencePlayer)
    (bind _asbp_mhplayer_controller (Utilities|Casting|CastToBP_MHPlayerController (Game|GetPlayerController 0)))
    (Default|ChangeQuestMode _asbp_mhplayer_controller)
    (Utilities|FlowControl|Delay 38.0)
    (Game|SpawnActorfromClass "/Game/Blueprints/BP_MHCharacterRathalos.BP_MHCharacterRathalos_C" (Math|Transform|MakeTransform (Math|Vector|MakeVector -10536.0 -29296.0 -6025.0) "0, 0, 0" "1.000000,1.000000,1.000000") "AdjustIfPossibleButAlwaysSpawn" 0 0)
    (bind _asbp_mhplayer_controller_2 (Utilities|Casting|CastToBP_MHPlayerController (Game|GetPlayerController 0)))
    (Default|ChangeFieldMode _asbp_mhplayer_controller_2)))

(event EventBeginPlay)

(event EventTick
  (params (DeltaSeconds :type Float%20%28single-precision%29)))

(fn ConstructionScript)