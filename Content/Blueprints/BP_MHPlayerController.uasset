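; Player controller that owns the HUD widgets for village, field and quest screens.
; BeginPlay sets game-only input, creates each widget once and shows the village HUD.
; Change-mode functions swap widgets on and off the viewport, with field mode also hiding the QuestLocator actor.
; Helper functions show quest popups, gating the dialog and acceptance widgets on a stored QuestProgress enum.
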(event EventBeginPlay
  (Input|SetInputModeGameOnly self false)
  (Utilities|FlowControl|Sequence
    (:then_0
      (bind _returnvalue (UserInterface|CreateWidget (Variables|Default|GetMHHUDWidgetClass)))
      (Variables|Default|SetMHHUDWidget _returnvalue))
    (:then_1
      (bind _returnvalue_2 (UserInterface|CreateWidget (Variables|Default|GetMHVillageHUDWidgetClass)))
      (bind _output_get (Variables|Default|SetMHVillageHUDWidget _returnvalue_2))
      (UserInterface|Viewport|AddtoViewport _output_get 0))
    (:then_2
      (bind _returnvalue_3 (UserInterface|CreateWidget (Variables|Default|GetMHQuestDialog%20HUDWidget%20Class)))
      (Variables|Default|SetMHQuestDialog%20HUDWidget _returnvalue_3))
    (:then_3
      (bind _returnvalue_4 (UserInterface|CreateWidget (Variables|Default|GetMHQuestAcceptance%20HUDWidget%20Class)))
      (Variables|Default|SetMHQuestAcceptance%20HUDWidget _returnvalue_4))
    (:then_4
      (bind _returnvalue_5 (UserInterface|CreateWidget (Variables|Default|GetMHQuestConfirm%20HUDWidget%20Class)))
      (Variables|Default|SetMHQuestConfirm%20HUDWidget _returnvalue_5))
    (:then_5
      (bind _returnvalue_6 (UserInterface|CreateWidget (Variables|Default|GetMHQuestReady%20HUDWidget%20Class)))
      (Variables|Default|SetMHQuestReady%20HUDWidget _returnvalue_6))
    (:then_6
      (bind _returnvalue_7 (UserInterface|CreateWidget (Variables|Default|GetMHCurrentQuest%20HUDWidget%20Class)))
      (Variables|Default|SetMHCurrentQuest%20HUDWidget _returnvalue_7))))

(fn ConstructionScript)

(fn ChangeVillageMode
  (Widget|RemovefromParent (Variables|Default|GetMHHUDWidget))
  (UserInterface|Viewport|AddtoViewport (Variables|Default|GetMHVillageHUDWidget) 0)
  (Widget|RemovefromParent (Variables|Default|GetMHQuestDialog%20HUDWidget))
  (Widget|RemovefromParent (Variables|Default|GetMHQuestAcceptance%20HUDWidget))
  (Widget|RemovefromParent (Variables|Default|GetMHQuestConfirm%20HUDWidget))
  (Widget|RemovefromParent (Variables|Default|GetMHQuestReady%20HUDWidget))
  (Widget|RemovefromParent (Variables|Default|GetMHCurrentQuest%20HUDWidget))
  (UserInterface|Viewport|AddtoViewport (Variables|Default|GetMHCurrentQuest%20HUDWidget) 0))

(fn ChangeFieldMode
  (Widget|RemovefromParent (Variables|Default|GetMHVillageHUDWidget))
  (UserInterface|Viewport|AddtoViewport (Variables|Default|GetMHHUDWidget) 0)
  (Widget|RemovefromParent (Variables|Default|GetMHQuestReady%20HUDWidget))
  (Widget|RemovefromParent (Variables|Default|GetMHCurrentQuest%20HUDWidget))
  (bind _returnvalue (Actor|GetActorOfClass "/Game/Blueprints/QuestLocator.QuestLocator_C"))
  (Default|SetVisible _returnvalue false))

(fn ChangeQuestMode
  (Widget|RemovefromParent (Variables|Default|GetMHVillageHUDWidget))
  (Widget|RemovefromParent (Variables|Default|GetMHHUDWidget))
  (Widget|RemovefromParent (Variables|Default|GetMHCurrentQuest%20HUDWidget)))

(fn SetQuestEnum
  (params (QuestProgress :type QuestProgress%20Enum :default "NewEnumerator0"))
  (Variables|Default|SetQuestProgress QuestProgress))

(fn AddUtusiDialog
  (if (Utilities|Enum|Equal(Enum) (Variables|Default|GetQuestProgress) "NewEnumerator0")
    (UserInterface|Viewport|AddtoViewport (Variables|Default|GetMHQuestDialog%20HUDWidget) 0)))

(fn AddQuestAcceptance
  (if (Utilities|Enum|Equal(Enum) (Variables|Default|GetQuestProgress) "NewEnumerator1")
    (UserInterface|Viewport|AddtoViewport (Variables|Default|GetMHQuestAcceptance%20HUDWidget) 0)))

(fn AddQuestConfirm
  (UserInterface|Viewport|AddtoViewport (Variables|Default|GetMHQuestConfirm%20HUDWidget) 0))

(fn CancleQuestConfirm
  (Widget|RemovefromParent (Variables|Default|GetMHQuestConfirm%20HUDWidget)))

(fn AddQuestReady
  (UserInterface|Viewport|AddtoViewport (Variables|Default|GetMHQuestReady%20HUDWidget) 0))

(fn QuestEnumCheck
  (params (QuestProgress :type QuestProgress%20Enum :default "NewEnumerator0"))
  (return (Utilities|Enum|Equal(Enum) QuestProgress (Variables|Default|GetQuestProgress))))