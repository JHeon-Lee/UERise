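; Rathalos boss monster character for a Monster Hunter-style game, with hit reactions, HUD monster icons, carving pickup on death and targeting of attackers.
; Point damage scales by the hardness of the nearest bone, shows damage numbers, and feeds part-break, tail-cut, stun and capture stats.
; Dragon riding has the player controller possess the monster for movement, evade and wall-slam rush, then hands it back to AI.
; Event hooks drive fire attacks, roar trace and anger/paralysis effects.
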(event OnComponentBeginOverlap(PickupTrigger)
  (params (OverlappedComponent :type Primitive%20Component%20Object%20Reference) (OtherActor :type Actor%20Object%20Reference) (OtherComp :type Primitive%20Component%20Object%20Reference) (OtherBodyIndex :type Integer) (bFromSweep :type Boolean) (SweepResult :type Hit%20Result%20Structure%20%28by%20ref%29))
  (bind _returnvalue (Class|MHRathalosStatComponent|IsHpZero (Variables|Default|GetStat)))
  (if _returnvalue
    (Utilities|FlowControl|Sequence
      (:then_0
        (bind _asbpi_is_player (Utilities|Casting|CastToBPI_IsPlayer OtherActor))
        (bind _bool (Default|IsPlayer _asbpi_is_player))
        (if (and _bool (not (Variables|Default|GetPicked)))
          (Rendering|SetVisibility (Variables|Default|GetWidget) true false)))
      (:then_1
        (bind _asreal_utusi (Utilities|Casting|CastToRealUtusi OtherActor))
        (if (and (Pawn|IsPlayerControlled _asreal_utusi) (Utilities|IsValid _asreal_utusi))
          (Default|SetNearProp _asreal_utusi self "갈무리"))))))

(event OnComponentEndOverlap(PickupTrigger)
  (params (OverlappedComponent :type Primitive%20Component%20Object%20Reference) (OtherActor :type Actor%20Object%20Reference) (OtherComp :type Primitive%20Component%20Object%20Reference) (OtherBodyIndex :type Integer))
  (bind _returnvalue (Class|MHRathalosStatComponent|IsHpZero (Variables|Default|GetStat)))
  (if _returnvalue
    (bind _asbpi_is_player (Utilities|Casting|CastToBPI_IsPlayer OtherActor))
    (bind _bool (Default|IsPlayer _asbpi_is_player))
    (if _bool
      (Default|SetNearProp (stale OnComponentBeginOverlap(PickupTrigger) _asreal_utusi) 0 "")
      (Rendering|SetVisibility (Variables|Default|GetWidget) false false))))

(event Input|EnhancedActionEvents|EnhancedInputActionIA_Move
  (params (ActionValue :type Vector%202D%20Structure) (ElapsedSeconds :type Float%20%28double-precision%29) (TriggeredSeconds :type Float%20%28double-precision%29) (InputAction :type Input%20Action%20Object%20Reference :default "/Game/ThirdPerson/Input/Actions/IA_Move.IA_Move"))
  ;[1 1 1] 용조종 Move
  (:Triggered
    (Pawn|Input|AddControllerYawInput (* (.x ActionValue) 0.3))
    (if (> (.y ActionValue) 0.0)
      (Variables|/Script/Engine.MovementComponent|SetVelocity (Variables|Character|GetCharacterMovement) (* (Math|Vector|GetForwardVector (Math|Rotator|MakeRotator 0.0 0.0 (.yaw (Pawn|GetControlRotation :!class /Script/Engine.Pawn)))) (* (.y ActionValue) 6e+02)))))
  (:Canceled
    (Variables|/Script/Engine.MovementComponent|SetVelocity (Variables|Character|GetCharacterMovement) "0, 0, 0" :!label _label))
  (:Completed
    (goto _label)))

(event Input|EnhancedActionEvents|EnhancedInputActionIA_B
  (params (ActionValue :type Boolean) (ElapsedSeconds :type Float%20%28double-precision%29) (TriggeredSeconds :type Float%20%28double-precision%29) (InputAction :type Input%20Action%20Object%20Reference :default "/Game/InputSystem/IA_B.IA_B"))
  (bind _playercharacterref (Variables|Default|GetPlayerCharacterRef))
  ;[1 1 1] 용조종 돌진이탈
  (:Started
    (Components|Capsule|SetCapsuleHalfHeight (Variables|Default|GetCapsuleComponent) 3e+02 true)
    (Animation|Montage|PlayMontage (Variables|Character|GetMesh) "/Game/Animations/AM_DragonRideRush.AM_DragonRideRush"
      (:OnCompleted
        (Pawn|Possess (Game|GetPlayerController 0) _playercharacterref)
        (Transformation|DetachFromActor _playercharacterref "KeepWorld" "KeepWorld" "KeepRelative")
        (Pawn|Components|CharacterMovement|SetMovementMode (Variables|/Script/Engine.Character|GetCharacterMovement _playercharacterref) "MOVE_Walking" 0)
        (Transformation|SetActorLocationAndRotation _playercharacterref (+ (Transformation|GetSocketLocation (Variables|Character|GetMesh) "DragonRideSocket") "300.000000,300.000000,400.000000"))
        (Animation|Montage|PlayMontage (Variables|Character|GetMesh) "/Game/Animations/AM_DragonRideKnockDown.AM_DragonRideKnockDown"
          (:OnCompleted
            (Pawn|Possess (Variables|Default|GetAIController) self)))))))

(event Input|EnhancedActionEvents|EnhancedInputActionIA_A
  (params (ActionValue :type Boolean) (ElapsedSeconds :type Float%20%28double-precision%29) (TriggeredSeconds :type Float%20%28double-precision%29) (InputAction :type Input%20Action%20Object%20Reference :default "/Game/InputSystem/IA_A.IA_A"))
  ;[1 1 1] 용조종 회피
  (:Started
    (if (and (> (Variables|Default|GetEvadeCount) 0) (Variables|Default|GetCanEvade))
      (Variables|Default|SetCanEvade false)
      (bind _result (Math|Integer|DecrementInt (Variables|Default|GetEvadeCount))
        (:%20%20
          (Variables|Default|SetEvadeCount _result)
          (Animation|Montage|PlayMontage (Variables|Character|GetMesh) "/Game/Animations/AM_DragonRideEvade.AM_DragonRideEvade"))))))

(event EventSetFirebreath
  (Niagara|SpawnSystematLocation "/Game/M5VFXVOL2/Niagara/Explosion/NFire_Exp_03.NFire_Exp_03" (Transformation|GetWorldLocation (Variables|Default|GetFireEffectArrow)) (Transformation|GetActorRotation self) "0.500000,0.500000,0.500000")
  (bind _returnvalue (Game|SpawnActorfromClass "/Game/Blueprints/BP_Firebreath.BP_Firebreath_C" (Math|Transform|MakeTransform (Transformation|GetWorldLocation (Variables|Default|GetFirebreathArrow)) "0, 0, 0" "1.000000,1.000000,1.000000") "AlwaysSpawn" 0 0))
  (Variables|Default|SetFireBreath _returnvalue)
  (Transformation|AttachComponentToComponent _returnvalue (Variables|Default|GetFirebreathArrow) "None" "KeepWorld" "KeepRelative" "KeepRelative" true))

(event EventSetFireball
  (bind _firearrow (Variables|Default|GetFireArrow))
  (Niagara|SpawnSystematLocation "/Game/M5VFXVOL2/Niagara/Explosion/NFire_Exp_03.NFire_Exp_03" (Transformation|GetWorldLocation (Variables|Default|GetFireEffectArrow)) (Transformation|GetActorRotation) "0.500000,0.500000,0.500000")
  (bind _returnvalue (Game|SpawnActorfromClass "/Game/Blueprints/BP_Fireball2.BP_Fireball2_C" (Math|Transform|MakeTransform (Transformation|GetWorldLocation _firearrow) (Transformation|GetActorRotation) "1.000000,1.000000,1.000000") "AlwaysSpawn" 0 0))
  (Utilities|IsValid _returnvalue
    (:Is%20Valid
      (Variables|/Script/Engine.MovementComponent|SetVelocity (Variables|/Game/Blueprints/BP_Fireball2.BP_Fireball2_C|GetProjectileMovement _returnvalue) (* (Math|Vector|GetForwardVector _firearrow) 2e+03)))))

(event EventSetFirebreath2
  (Niagara|SpawnSystematLocation "/Game/M5VFXVOL2/Niagara/Explosion/NFire_Exp_03.NFire_Exp_03" (Transformation|GetWorldLocation (Variables|Default|GetFireEffectArrow)) (Transformation|GetActorRotation self) "0.500000,0.500000,0.500000")
  (bind _returnvalue (Game|SpawnActorfromClass "/Game/Blueprints/BP_Firebreath2.BP_Firebreath2_C" (Math|Transform|MakeTransform (Transformation|GetWorldLocation (Variables|Default|GetFirebreathArrow2)) "0, 0, 0" "1.000000,1.000000,1.000000") "AlwaysSpawn" 0 0))
  (Variables|Default|SetFireBreath2 _returnvalue)
  (Transformation|AttachComponentToComponent _returnvalue (Variables|Default|GetFirebreathArrow2) "None" "KeepWorld" "KeepRelative" "KeepRelative" true))

(event EventTailCut
  (bind _bp_mhtail (Variables|Default|GetBP_MHTail))
  (Rendering|Material|SetScalarParameterValue "/Game/ImportSource/RathalosSK/MPC_Damage.MPC_Damage" "Opacity" 1.0 :!class /Script/Engine.KismetMaterialLibrary)
  (Transformation|DetachFromComponent _bp_mhtail "KeepWorld" "KeepWorld" "KeepRelative" true)
  (bind _asbpi_set_tail_cut (Utilities|Casting|CastToBPI_SetTailCut (Variables|/Script/Engine.ChildActorComponent|GetChildActor _bp_mhtail)))
  (Default|TailCut _asbpi_set_tail_cut))

(event EventSetDragonRiding
  (if (Variables|Default|GetbIsDragonRiding)
    (Variables|Default|SetbIsDragonRiding false)
    (else
      (Variables|Default|SetbIsDragonRiding true))))

(event EventSetPlayerRide
  (bind _returnvalue (Game|GetPlayerCharacter 0))
  (bind _returnvalue_2 (Game|GetPlayerController 0))
  (bind _returnvalue_3 (PlayerController|LocalPlayerSubsystems|GetEnhancedInputLocalPlayerSubsystem _returnvalue_2))
  ;[1 1 1] 용조종 인터페이스
  (if (Variables|Default|GetbIsDragonRiding)
    (Variables|Default|SetbIsDragonRiding false)
    (Components|DestroyComponent (Variables|Default|GetCanRideWidget))
    (Variables|Default|SetPlayerCharacterRef _returnvalue)
    (Pawn|Components|CharacterMovement|SetMovementMode (Variables|/Script/Engine.Character|GetCharacterMovement _returnvalue) "MOVE_Flying" 0)
    (Transformation|AttachComponentToComponent _returnvalue (Variables|Character|GetMesh) "DragonRideSocket" "KeepWorld" "KeepWorld" "KeepRelative" true)
    (Transformation|SetActorLocationAndRotation _returnvalue (Transformation|GetSocketLocation (Variables|Character|GetMesh) "DragonRideSocket") (Transformation|GetActorRotation))
    (Animation|StopAnimMontage "/Game/Animations/AM_DragonRideReady.AM_DragonRideReady")
    (Pawn|Components|CharacterMovement|SetMovementMode (Variables|Character|GetCharacterMovement) "MOVE_Flying" 0)
    (CameraFades|StartCameraFade :self (Variables|/Script/Engine.PlayerController|GetPlayerCameraManager (Game|GetPlayerController 0)) :ToAlpha 1.0 :Duration 1.0 :bHoldWhenFinished true)
    (Animation|Montage|PlayMontage (Variables|Character|GetMesh) "/Game/Animations/AM_Fly.AM_Fly"
      (:OnCompleted
        (Pawn|Possess _returnvalue_2 self)
        (CameraFades|StartCameraFade :self (Variables|/Script/Engine.PlayerController|GetPlayerCameraManager _returnvalue_2) :FromAlpha 1.0 :Duration 1.0)
        (bind _asmhplayer_controller (Utilities|Casting|CastToMHPlayerController _returnvalue_2))
        (bind _aswbp_mhhud (Utilities|Casting|CastToWBP_MHHUD (Variables|/Script/UERise.MHPlayerController|GetMHHUDWidget _asmhplayer_controller)))
        (Class|Image|SetOpacity (Variables|/Game/Characters/Utusi/UI/WBP_MonsterIcon.WBP_MonsterIcon_C|GetDragonRideIcon (Variables|/Game/Characters/Utusi/UI/WBP_MHHUD.WBP_MHHUD_C|GetWBP_MonsterIcon _aswbp_mhhud)) 1.0)
        (Variables|/Script/UMG.Widget|SetVisibility (Variables|/Game/Characters/Utusi/UI/WBP_MHHUD.WBP_MHHUD_C|GetWBP_ItemFrame _aswbp_mhhud) "Hidden")
        (Variables|/Script/UMG.Widget|SetVisibility (Variables|/Game/Characters/Utusi/UI/WBP_MHHUD.WBP_MHHUD_C|GetWBP_DragonRideControl _aswbp_mhhud) "Visible")
        (Variables|/Script/UMG.Widget|SetVisibility (Variables|/Game/Characters/Utusi/UI/WBP_MHHUD.WBP_MHHUD_C|GetWBP_DragonRideUI _aswbp_mhhud) "Visible")
        (Utilities|IsValid _returnvalue_3
          (:Is%20Valid
            (Input|AddMappingContext _returnvalue_3 "/Game/InputSystem/UtusiMappingContext.UtusiMappingContext" 0 "(bIgnoreAllPressedKeysUntilRelease=True,bForceImmediately=False)")
            (Pawn|Components|CharacterMovement|SetMovementMode (Variables|Character|GetCharacterMovement) "MOVE_Flying" 0)
            (Components|Capsule|SetCapsuleHalfHeight (Variables|Default|GetCapsuleComponent) 6e+02 true)))))))

(event EventSetWalking
  (Pawn|Components|CharacterMovement|SetMovementMode (Variables|Character|GetCharacterMovement) "MOVE_Walking" 0))

(event EventSetFlying
  (Pawn|Components|CharacterMovement|SetMovementMode (Variables|Character|GetCharacterMovement) "MOVE_Flying" 0))

(event EventSetAIRun
  (Pawn|Possess (Variables|Default|GetAIController) self))

(event EventSetParalizeEffecton
  (Rendering|SetVisibility (Variables|Default|GetParalyzeTrapEft) true false))

(event EventSetParalizeEffectOff
  (Rendering|SetVisibility (Variables|Default|GetParalyzeTrapEft) false false))

(event EventSetWallHit
  (if (Variables|Default|GetCanWallHit)
    (Variables|Default|SetCanWallHit false)
    (else
      (Variables|Default|SetCanWallHit true))))

(event EventSetFirebreathOff
  (params (ScaleVec :type Vector :default "0, 0, 0"))
  (bind _firebreath (Variables|Default|GetFireBreath))
  (Niagara|SpawnSystematLocation "/Game/M5VFXVOL2/Niagara/Explosion/NFire_Exp_03.NFire_Exp_03" (Transformation|GetWorldLocation (Variables|Default|GetFireEffectArrow)) (Transformation|GetActorRotation self) ScaleVec)
  (if (Utilities|IsValid _firebreath)
    (Actor|DestroyActor _firebreath)))

(event EventSetEvade
  (if (Variables|Default|GetCanEvade)
    (Variables|Default|SetCanEvade false)
    (else
      (Variables|Default|SetCanEvade true))))

(event Collision|EventActorBeginOverlap
  (params (OtherActor :type Actor%20Object%20Reference))
  (bind _returnvalue (Transformation|GetActorLocation))
  (bind _playercharacterref (Variables|Default|GetPlayerCharacterRef))
  (bind _canridewidget (Variables|Default|GetCanRideWidget))
  (Utilities|FlowControl|Sequence
    (:then_0
      ;[1 1 1] 용조종 벽꿍
      (if (and (Variables|Default|GetCanWallHit) (Actor|ActorHasTag OtherActor "CanWallHit"))
        (Variables|Default|SetCanWallHit false)
        (Camera|PlayWorldCameraShake "/Game/Blueprints/CAM_SHAKE.CAM_SHAKE_C" _returnvalue 0.0 2e+03)
        (Effects|SpawnEmitteratLocation "/Game/MarketContent/Realistic_Starter_VFX_Pack_Vol2/Particles/Destruction/P_Destruction_Building_A.P_Destruction_Building_A" _returnvalue "0, 0, 0" "4.000000,4.000000,4.000000")
        (Animation|StopAnimMontage "/Game/Animations/AM_DragonRideRush.AM_DragonRideRush")
        (Animation|Montage|PlayMontage (Variables|Character|GetMesh) "/Game/Animations/AM_DragonRideWallHit.AM_DragonRideWallHit"
          (:OnCompleted
            ;[1 1 1] 용조종 돌진이탈
            (Pawn|Possess (Game|GetPlayerController 0) _playercharacterref)
            (Transformation|DetachFromActor _playercharacterref "KeepWorld" "KeepWorld" "KeepRelative")
            (Pawn|Components|CharacterMovement|SetMovementMode (Variables|/Script/Engine.Character|GetCharacterMovement _playercharacterref) "MOVE_Walking" 0)
            (Transformation|SetActorLocationAndRotation _playercharacterref (+ (Transformation|GetSocketLocation (Variables|Character|GetMesh) "DragonRideSocket") "300.000000,300.000000,400.000000"))
            (Animation|Montage|PlayMontage (Variables|Character|GetMesh) "/Game/Animations/AM_DragonRideKnockDown.AM_DragonRideKnockDown"
              (:OnCompleted
                (Pawn|Possess (Variables|Default|GetAIController) self)))))))
    (:then_1
      ;[1 1 1] 용조종 가능 UI 띄우기
      (if (and (Variables|Default|GetbIsDragonRiding) (Utilities|DoesObjectImplementInterface OtherActor "/Game/Blueprints/BPI_IsPlayer.BPI_IsPlayer_C"))
        (Utilities|IsValid _canridewidget
          (:Is%20Valid
            (Rendering|SetVisibility _canridewidget true false)
            (Utilities|FlowControl|Delay 5.5)
            (Utilities|IsValid _canridewidget
              (:Is%20Valid
                (Rendering|SetVisibility _canridewidget false false)))))))))

(event Game|Damage|EventPointDamage
  (params (Damage :type Float%20%28single-precision%29) (DamageType :type Damage%20Type%20Object%20Reference) (HitLocation :type Vector :default "0, 0, 0") (HitNormal :type Vector :default "0, 0, 0") (HitComponent :type Primitive%20Component%20Object%20Reference) (BoneName :type Name :default "None") (ShotFromDirection :type Vector :default "0, 0, 0") (InstigatedBy :type Controller%20Object%20Reference) (DamageCauser :type Actor%20Object%20Reference) (HitInfo :type Hit%20Result%20Structure%20%28by%20ref%29))
  (bind _location (Collision|BreakHitResult HitInfo))
  (bind _stat (Variables|Default|GetStat))
  (Utilities|Casting|CastToCriticalDamageType DamageType
    (:then
      (Variables|Default|SetCritical true))
    (:CastFailed
      (Variables|Default|SetCritical false)))
  (for _array_element (Variables|Default|GetRathalosPartsHardnessInfo)
    (if (Utilities|String|Contains (Utilities|String|ToString(Name) (.ReturnValue (Class|SkinnedMeshComponent|FindClosestBoneK2 (Variables|Character|GetMesh) _location 0.0))) (.bonename _array_element))
      ;[1 1 1] 상태이상 데미지타입 예외처리
      (bind _notailmenttype (CallFunction|CheckDamageType DamageType))
      (if _notailmenttype
        (if (>= (.hardness _array_element) 0.45)
          (if (Variables|Default|GetCritical)
            ;[1 1 1] 데미지 표기
            (Utilities|SpawnDynamicTextatWorld :Spawn%20Transform%20Location _location :Animation "NewEnumerator3" :Text%20Damage (Utilities|Text|ToText(Integer) (Math|Float|Round (* Damage (.hardness _array_element)))) :Font (Variables|Default|GetCritFont) :Font%20Color "(R=1.000000,G=0.298944,B=0.047060,A=1.000000)" :Font%202%20Color "(R=1.000000,G=0.070360,B=0.040915,A=1.000000)")
            (else
              (Utilities|SpawnDynamicTextatWorld :Spawn%20Transform%20Location _location :Animation "NewEnumerator3" :Text%20Damage (Utilities|Text|ToText(Integer) (Math|Float|Round (* Damage (.hardness _array_element)))) :Font (Variables|Default|GetNonCritFont) :Font%20Color "(R=1.000000,G=0.592295,B=0.000000,A=1.000000)")))
          (else
            (Utilities|SpawnDynamicTextatWorld :Spawn%20Transform%20Location _location :Animation "NewEnumerator3" :Text%20Damage (Utilities|Text|ToText(Integer) (Math|Float|Round (* Damage (.hardness _array_element)))) :Font (Variables|Default|GetNonCritFont) :Font%202%20Color "(R=1.000000,G=0.070360,B=0.040915,A=1.000000)"))))
      ;[1 1 1] 육질 적용된 데미지 스탯에 적용
      (bind _returnvalue (Class|MHRathalosStatComponent|ApplyDamage _stat (Math|Conversions|ToFloat(Integer) (Math|Float|Round (* Damage (.hardness _array_element))))))
      (bind _returnvalue_2 (Class|MHRathalosStatComponent|GetCurrentHp _stat))
      (Development|PrintString (Utilities|String|ToString(Float) _returnvalue_2))
      ;[0 0.5312 1] 경직 모션중 중복 방지
      (Utilities|FlowControl|Sequence
        (:then_0
          (bind _array_element_2 (Utilities|Array|ForEachLoopwithBreak (Variables|Default|GetDamagedMontages) :!label _label)
            (:LoopBody
              (if (Animation|Montage|MontageIsPlaying (Components|SkeletalMesh|GetAnimInstance (Variables|Character|GetMesh)) _array_element_2)
                (goto _label Break)))
            (:Completed
              (Utilities|FlowControl|Sequence
                (:then_0
                  (if (Utilities|String|Contains (.nearestpart _array_element) "Head")
                    (Class|MHRathalosStatComponent|ApplyHeadBreakRate (Variables|Default|GetStat) _returnvalue)
                    (bind _asmhdamage_type_tackle (Utilities|Casting|CastToMHDamageType_Tackle DamageType))
                    (Utilities|IsValid _asmhdamage_type_tackle
                      (:Is%20Valid
                        (Class|MHRathalosStatComponent|ApplyStunCount (Variables|Default|GetStat) 1.0)))))
                (:then_1
                  (if (Utilities|String|Contains (.nearestpart _array_element) "Leg")
                    (Class|MHRathalosStatComponent|ApplyLegBreakRate (Variables|Default|GetStat) _returnvalue)))
                (:then_2
                  (if (Utilities|String|Contains (.nearestpart _array_element) "Wing")
                    (Class|MHRathalosStatComponent|ApplyWingBreakRate (Variables|Default|GetStat) _returnvalue)))
                (:then_3
                  (if (Utilities|String|Contains (.nearestpart _array_element) "Tail")
                    (Class|MHRathalosStatComponent|ApplyTailCutRate (Variables|Default|GetStat) _returnvalue)))))))
        (:then_1
          (Utilities|FlowControl|Sequence
            (:then_0
              (Utilities|Casting|CastToMHDamageType_Capture DamageType)
              (bind _returnvalue_3 (Class|MHRathalosStatComponent|IsHp10Percent (Variables|Default|GetStat)))
              (if _returnvalue_3
                (Class|MHRathalosStatComponent|ApplyCaptureCount (Variables|Default|GetStat) 1.0)))
            (:then_1
              (Utilities|Casting|CastToMHDamageType_Flash DamageType)
              (if (Class|NavMovementComponent|IsFlying (Variables|Character|GetCharacterMovement))
                (Class|MHRathalosStatComponent|ApplyStunCount (Variables|Default|GetStat) 2.0)))
            (:then_2
              (Utilities|Casting|CastToMHDamageType_StunTrap DamageType)
              (Class|MHCharacterRathalos|SetStunTrapEffected))
            (:then_3
              ;[1 1 1] TODO : 수면속성
              (Utilities|Casting|CastToMHDamageType_Sleep DamageType))))))))

(event EventBeginPlay
  (Variables|Default|SetAIController (Pawn|GetController))
  ;[1 1 1] 일정시간 지나면 도망
  (Utilities|FlowControl|Delay 9e+01) ; 270
  (Variables|Default|Setb270secElapsed true)
  (Rendering|Material|SetVectorParameterValue "/Game/ImportSource/RathalosSK/MPC_AngerEye.MPC_AngerEye" "EyeEmissive" (Variables|Default|GetBlack%20Vec) :!class /Script/Engine.KismetMaterialLibrary)
  (Components|Activation|SetActive (Variables|Default|GetAngerFire) false false))

(event EventSetFirebreathOff2
  (bind _firebreath2 (Variables|Default|GetFireBreath2))
  (Niagara|SpawnSystematLocation "/Game/M5VFXVOL2/Niagara/Explosion/NFire_Exp_03.NFire_Exp_03" (Transformation|GetWorldLocation (Variables|Default|GetFireEffectArrow)) (Transformation|GetActorRotation self) "0.500000,0.500000,0.500000")
  (if (Utilities|IsValid _firebreath2)
    (Actor|DestroyActor _firebreath2)))

(event EventSetRadialBluron
  (bind _radialbluron (Timeline|Timeline Play)
    (:Update
      (Rendering|Material|SetScalarParameterValue "/Game/ImportSource/MPC_RadialBlur.MPC_RadialBlur" "Lerp Alpha" _radialbluron :!class /Script/Engine.KismetMaterialLibrary)
      (Utilities|FlowControl|Delay 1.5)
      (bind _radialbluroff (Timeline|Timeline_1 Play)
        (:Update
          (Rendering|Material|SetScalarParameterValue "/Game/ImportSource/MPC_RadialBlur.MPC_RadialBlur" "Lerp Alpha" _radialbluroff :!class /Script/Engine.KismetMaterialLibrary))))))

(event EventSetAngerEffecton
  (Rendering|Material|SetVectorParameterValue "/Game/ImportSource/RathalosSK/MPC_AngerEye.MPC_AngerEye" "EyeEmissive" (Variables|Default|GetRed%20Vec) :!class /Script/Engine.KismetMaterialLibrary)
  (Components|Activation|SetActive (Variables|Default|GetAngerFire) true false))

(event EventSetRoarAttackHitCheck
  (bind _mesh (Variables|Character|GetMesh))
  (bind _returnvalue (Transformation|GetSocketLocation _mesh "TongueSocket"))
  (bind _outhit (Collision|SphereTraceByChannel _returnvalue (+ _returnvalue "1000.000000,0.000000,0.000000") 1e+03 "TraceTypeQuery3" false 0 "ForOneFrame"))
  (bind _asbpi_is_player (Utilities|Casting|CastToBPI_IsPlayer (.HitActor (Collision|BreakHitResult _outhit))))
  (bind _bool (Default|IsPlayer _asbpi_is_player))
  (if _bool
    (Game|Damage|ApplyDamage (.HitActor (Collision|BreakHitResult _outhit)) 0.01 0 0 "/Script/UERise.MHDamageType_Roar")))

(event Game|Damage|EventAnyDamage
  (params (Damage :type Float%20%28single-precision%29) (DamageType :type Damage%20Type%20Object%20Reference) (InstigatedBy :type Controller%20Object%20Reference) (DamageCauser :type Actor%20Object%20Reference))
  (bind _returnvalue (Pawn|GetController))
  (bind _returnvalue_2 (Game|GetPlayerController 0))
  (bind _returnvalue_3 (AI|GetBlackboard _returnvalue))
  (Utilities|FlowControl|Sequence
    (:then_0
      ;[1 1 1] 채집 시
      (if (== (Utilities|GetClass DamageType) "/Game/Blueprints/BP_MHDamageType_Pickup.BP_MHDamageType_Pickup_C")
        (Utilities|FlowControl|Sequence
          (:then_0
            (Variables|Default|SetPicked true)
            (Rendering|SetVisibility (Variables|Default|GetWidget) false false))
          (:then_1
            (bind _asbpi_is_player (Utilities|Casting|CastToBPI_IsPlayer DamageCauser))
            (Default|PickupItem _asbpi_is_player (Variables|Default|GetItem))))))
    (:then_1
      ;[1 1 1] 우상단 HUD 아이콘
      (Utilities|FlowControl|Delay 0.1)
      (bind _returnvalue_4 (Class|MHRathalosStatComponent|IsHp10Percent (Variables|Default|GetStat)))
      (if _returnvalue_4
        (bind _asmhplayer_controller (Utilities|Casting|CastToMHPlayerController _returnvalue_2))
        (bind _aswbp_mhhud (Utilities|Casting|CastToWBP_MHHUD (Variables|/Script/UERise.MHPlayerController|GetMHHUDWidget _asmhplayer_controller)))
        (Class|Image|SetOpacity (Variables|/Game/Characters/Utusi/UI/WBP_MonsterIcon.WBP_MonsterIcon_C|GetHp10Icon (Variables|/Game/Characters/Utusi/UI/WBP_MHHUD.WBP_MHHUD_C|GetWBP_MonsterIcon _aswbp_mhhud)) 1.0)
        (else
          (bind _returnvalue_5 (Class|MHRathalosStatComponent|IsHpZero (Variables|Default|GetStat)))
          (if _returnvalue_5
            (bind _asmhplayer_controller_2 (Utilities|Casting|CastToMHPlayerController _returnvalue_2))
            (bind _aswbp_mhhud_2 (Utilities|Casting|CastToWBP_MHHUD (Variables|/Script/UERise.MHPlayerController|GetMHHUDWidget _asmhplayer_controller_2)))
            (Class|Image|SetOpacity (Variables|/Game/Characters/Utusi/UI/WBP_MonsterIcon.WBP_MonsterIcon_C|GetHp10Icon (Variables|/Game/Characters/Utusi/UI/WBP_MHHUD.WBP_MHHUD_C|GetWBP_MonsterIcon _aswbp_mhhud_2)) 0.0)
            (Variables|/Game/Characters/Utusi/UI/WBP_TargetMonsterName.WBP_TargetMonsterName_C|SetMonsterDead (Variables|/Game/Characters/Utusi/UI/WBP_MHHUD.WBP_MHHUD_C|GetWBP_TargetMonsterName _aswbp_mhhud_2) true)
            (Variables|/Game/Characters/Utusi/UI/WBP_RightSideAlarm.WBP_RightSideAlarm_C|SetMonsterDead (Variables|/Game/Characters/Utusi/UI/WBP_MHHUD.WBP_MHHUD_C|GetWBP_RightSideAlarm _aswbp_mhhud_2) true)))))
    (:then_2
      ;[1 1 1] 미탐지시 데미지 입으면 바로 타겟팅
      (Utilities|IsValid _returnvalue_3
        (:Is%20Valid
          (if (not (ScalableFloat|GetValueasBool _returnvalue_3 (Variables|Default|GetIsDetecting)))
            (bind _asbpi_is_player_2 (Utilities|Casting|CastToBPI_IsPlayer DamageCauser))
            (bind _bool (Default|IsPlayer _asbpi_is_player_2))
            (if _bool
              (AI|Components|Blackboard|SetValueasObject _returnvalue_3 (Variables|Default|GetTarget) DamageCauser)
              (AI|Components|Blackboard|SetValueasBool _returnvalue_3 (Variables|Default|GetIsDetecting) true))))))))

(fn ConstructionScript)

(fn SpawnFloatingDmg
  (params (Damage :type Float%20%28double-precision%29) (IsEffective :type Boolean) (Location :type Vector))
  (bind _returnvalue (Math|Float|Round Damage))
  (bind _returnvalue_2 (Utilities|Text|ToText(Integer) _returnvalue))
  (if IsEffective
    (Utilities|SpawnDynamicTextatWorld :Spawn%20Transform%20Location Location :Animation "NewEnumerator3" :Text%20Damage _returnvalue_2 :Font (Variables|Default|GetEffectiveDmg) :Font%20Color "(R=1.000000,G=0.592295,B=0.000000,A=1.000000)")
    (else
      (Utilities|SpawnDynamicTextatWorld :Spawn%20Transform%20Location Location :Animation "NewEnumerator3" :Text%20Damage _returnvalue_2 :Font (Variables|Default|GetNotEffectiveDmg) :Font%20Color "(R=0.526042,G=0.526042,B=0.526042,A=1.000000)"))))

(fn CheckDamageType
  (params (DamageType :type Damage%20Type%20Object%20Reference))
  (Utilities|Casting|CastToMHDamageType_Flash DamageType
    (:then
      (return false))
    (:CastFailed
      (Utilities|Casting|CastToMHDamageType_StunTrap DamageType
        (:then
          (return false))
        (:CastFailed
          (Utilities|Casting|CastToMHDamageType_Capture DamageType
            (:then
              (return false))
            (:CastFailed
              (return true))))))))

(fn GetCanDragonRide
  (return (Variables|Default|GetbIsDragonRiding)))

(fn IsMonster
  (return true))