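; QuestLocator is an actor with a widget component, by its name a marker for quest locations.
; On BeginPlay it rotates the widget once to face the player camera, then plays a timeline.
; Each timeline update adds the Zlocation track value to the actor's current height, so the vertical offset accumulates.
; SetVisible shows or hides the widget without propagating to child components.
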(event EventBeginPlay
  (bind _returnvalue (Transformation|GetActorLocation))
  (bind _widget (Variables|Default|GetWidget))
  (Transformation|SetWorldRotation _widget (Math|Rotator|FindLookatRotation (Transformation|GetWorldLocation _widget) (Transformation|GetWorldLocation (Variables|/Script/Engine.PlayerCameraManager|GetTransformComponent (Game|GetPlayerCameraManager 0)))) false false)
  (bind _zlocation (Timeline|Timeline Play)
    (:Update
      (Transformation|SetActorLocation (Math|Vector|MakeVector (.x _returnvalue) (.y _returnvalue) (+ (.z _returnvalue) _zlocation)) false false))))

(fn ConstructionScript)

(fn SetVisible
  (params (bool :type Boolean))
  (Rendering|SetVisibility (Variables|Default|GetWidget) bool false))