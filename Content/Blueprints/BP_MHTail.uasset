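; BP_MHTail is a tail prop that, once cut, falls under physics and can be carved ("갈무리") for a Tail item.
; TailCut turns on physics and gravity, adds a slight upward velocity and enables the overlap prompt.
; The box overlap shows a widget until picked and registers the tail as a player-controlled RealUtusi's nearby prop.
; Any damage marks it picked, hides the widget and calls PickupItem on the causer through BPI_IsPlayer.
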(event OnComponentBeginOverlap(Box)
  (params (OverlappedComponent :type Primitive%20Component%20Object%20Reference) (OtherActor :type Actor%20Object%20Reference) (OtherComp :type Primitive%20Component%20Object%20Reference) (OtherBodyIndex :type Integer) (bFromSweep :type Boolean) (SweepResult :type Hit%20Result%20Structure%20%28by%20ref%29))
  (if (Variables|Default|GetCut)
    (Utilities|FlowControl|Sequence
      (:then_0
        (if (not (Variables|Default|GetPicked))
          (Rendering|SetVisibility (Variables|Default|GetWidget) true false)))
      (:then_1
        (bind _asreal_utusi (Utilities|Casting|CastToRealUtusi OtherActor))
        (if (and (Pawn|IsPlayerControlled _asreal_utusi) (Utilities|IsValid _asreal_utusi))
          (Default|SetNearProp _asreal_utusi self "갈무리"))))))

(event OnComponentEndOverlap(Box)
  (params (OverlappedComponent :type Primitive%20Component%20Object%20Reference) (OtherActor :type Actor%20Object%20Reference) (OtherComp :type Primitive%20Component%20Object%20Reference) (OtherBodyIndex :type Integer))
  (Rendering|SetVisibility (Variables|Default|GetWidget) false false)
  (Utilities|IsValid (stale OnComponentBeginOverlap(Box) _asreal_utusi)
    (:Is%20Valid
      (Default|SetNearProp (stale OnComponentBeginOverlap(Box) _asreal_utusi) 0 ""))))

(event EventBeginPlay
  (bind _widget (Variables|Default|GetWidget))
  (Transformation|SetWorldRotation _widget (Math|Rotator|FindLookatRotation (Transformation|GetWorldLocation _widget) (Transformation|GetWorldLocation (Variables|/Script/Engine.PlayerCameraManager|GetTransformComponent (Game|GetPlayerCameraManager 0)))) false false))

(event EventTailCut
  (bind _cube (Variables|Default|GetCube))
  (bind _projectilemovement (Variables|Default|GetProjectileMovement))
  (Physics|SetSimulatePhysics _cube true)
  (Physics|SetEnableGravity _cube true)
  (Collision|SetCollisionProfileName _cube "PhysicsBody" true :!class /Script/Engine.PrimitiveComponent)
  (Variables|/Script/Engine.ProjectileMovementComponent|SetProjectileGravityScale _projectilemovement 1.0)
  (Variables|/Script/Engine.MovementComponent|SetVelocity _projectilemovement "0.000000,0.000000,10.000000")
  (Variables|Default|SetCut true))

(event Game|Damage|EventAnyDamage
  (params (Damage :type Float%20%28single-precision%29) (DamageType :type Damage%20Type%20Object%20Reference) (InstigatedBy :type Controller%20Object%20Reference) (DamageCauser :type Actor%20Object%20Reference))
  (Utilities|FlowControl|Sequence
    (:then_0
      (Variables|Default|SetPicked true)
      (Rendering|SetVisibility (Variables|Default|GetWidget) false false))
    (:then_1
      (bind _asbpi_is_player (Utilities|Casting|CastToBPI_IsPlayer DamageCauser))
      (Default|PickupItem _asbpi_is_player (Variables|Default|GetTail)))))

(fn ConstructionScript)