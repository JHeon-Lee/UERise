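; BP_LevelChange is a level transition trigger that moves the RealUtusi character to another streamed level, open only while the quest is accepted.
; A Plane overlap checks the player controller's QuestProgress, then shows its loading-screen widget and plays a sound, both only once via DoOnce.
; It then loads the target streaming level, moves the character to the WarpPoint's location and rotation, and unloads the previous level.
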(event OnComponentBeginOverlap(Plane)
  (params (OverlappedComponent :type Primitive%20Component%20Object%20Reference) (OtherActor :type Actor%20Object%20Reference) (OtherComp :type Primitive%20Component%20Object%20Reference) (OtherBodyIndex :type Integer) (bFromSweep :type Boolean) (SweepResult :type Hit%20Result%20Structure%20%28by%20ref%29))
  (bind _asreal_utusi (Utilities|Casting|CastToRealUtusi OtherActor))
  (Utilities|IsValid _asreal_utusi
    (:Is%20Valid
      (Variables|Default|SetAs%20Real%20Utusi _asreal_utusi)
      ;[1 1 1] 퀘스트 받은 상태에서만 입장 가능
      (bind _asbp_mhplayer_controller (Utilities|Casting|CastToBP_MHPlayerController (Game|GetPlayerController 0)))
      (Variables|Default|SetAs%20BP%20MHPlayer%20Controller _asbp_mhplayer_controller)
      (if (Utilities|Enum|Equal(Enum) (Variables|/Game/Blueprints/BP_MHPlayerController.BP_MHPlayerController_C|GetQuestProgress _asbp_mhplayer_controller) "NewEnumerator2")
        (Utilities|FlowControl|Sequence
          (:then_0
            (Utilities|FlowControl|DoOnce false
              (:Completed
                (UserInterface|Viewport|AddtoViewport (Variables|/Game/Blueprints/BP_MHPlayerController.BP_MHPlayerController_C|GetLodingScenes (Variables|Default|GetAs%20BP%20MHPlayer%20Controller)) 0)
                (Audio|PlaySound2D "/Game/ImportSource/Sound/UI/ui100/UILodingscene.UILodingscene" 1.0 1.0 0.0 0 0))))
          (:then_1
            (Class|GameplayStatics|LoadStreamLevelbySoftObjectPtr (Variables|Default|GetLevelLoad) true false)
            (Transformation|SetActorLocation (Variables|Default|GetAs%20Real%20Utusi) (Transformation|GetWorldLocation (Variables|Default|GetWarpPoint)) false false)
            (Transformation|SetActorRotation (Variables|Default|GetAs%20Real%20Utusi) (Transformation|GetWorldRotation (Variables|Default|GetWarpPoint)))
            (Class|GameplayStatics|UnloadStreamLevelbySoftObjectPtr (Variables|Default|GetLevelUnload) false)))))))

(event EventBeginPlay)

(event Collision|EventActorBeginOverlap
  (params (OtherActor :type Actor%20Object%20Reference)))

(event EventTick
  (params (DeltaSeconds :type Float%20%28single-precision%29)))

(fn ConstructionScript)