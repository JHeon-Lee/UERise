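; Anim notify state that shows the right-side alarm on the player HUD for the duration of its window in an animation.
; On begin it sets the WBPRightSideAlarm widget in WBP_MHHUD to visible, and on end it hides it.
; The HUD is always reached through player controller 0, regardless of which mesh plays the animation.
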(fn ReceivedNotifyEnd
  (params (MeshComp :type Skeletal%20Mesh%20Component%20Object%20Reference) (Animation :type Anim%20Sequence%20Base%20Object%20Reference) (EventReference :type Anim%20Notify%20Event%20Reference%20Structure%20%28by%20ref%29))
  (bind _asmhplayer_controller (Utilities|Casting|CastToMHPlayerController (Game|GetPlayerController MeshComp)))
  (bind _aswbp_mhhud (Utilities|Casting|CastToWBP_MHHUD (Variables|/Script/UERise.MHPlayerController|GetMHHUDWidget _asmhplayer_controller)))
  (Variables|/Script/UMG.Widget|SetVisibility (Variables|/Game/Characters/Utusi/UI/WBP_MHHUD.WBP_MHHUD_C|GetWBP_RightSideAlarm _aswbp_mhhud) "Hidden")
  (return false))

(fn ReceivedNotifyBegin
  (params (MeshComp :type Skeletal%20Mesh%20Component%20Object%20Reference) (Animation :type Anim%20Sequence%20Base%20Object%20Reference) (TotalDuration :type Float%20%28single-precision%29) (EventReference :type Anim%20Notify%20Event%20Reference%20Structure%20%28by%20ref%29))
  (bind _asmhplayer_controller (Utilities|Casting|CastToMHPlayerController (Game|GetPlayerController MeshComp)))
  (bind _aswbp_mhhud (Utilities|Casting|CastToWBP_MHHUD (Variables|/Script/UERise.MHPlayerController|GetMHHUDWidget _asmhplayer_controller)))
  (Variables|/Script/UMG.Widget|SetVisibility (Variables|/Game/Characters/Utusi/UI/WBP_MHHUD.WBP_MHHUD_C|GetWBP_RightSideAlarm _aswbp_mhhud) "Visible")
  (return false))