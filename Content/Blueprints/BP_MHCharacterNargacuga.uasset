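; Nargacuga monster character that plays a scripted turf war and then leaves the map.
; On BeginPlay it plays the turf war montage and, when that completes, uses AIMoveTo to head for a hardcoded world location.
; On arrival it destroys itself and dims its monster icon on the player's HUD, while a failed move only prints a debug message.
; A helper function returns ground speed as the length of the movement velocity.
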(event EventBeginPlay
  (Animation|Montage|PlayMontage (Variables|Character|GetMesh) "/Game/Animations/AM_NargaTurfWar.AM_NargaTurfWar"
    (:OnCompleted
      (AI|AIMoveTo self "-11570.000000,-42960.000000,-8105.000000" 0 1e+03 false
        (:OnSuccess
          (Actor|DestroyActor)
          (bind _asmhplayer_controller (Utilities|Casting|CastToMHPlayerController (Game|GetPlayerController 0)))
          (bind _aswbp_mhhud (Utilities|Casting|CastToWBP_MHHUD (Variables|/Script/UERise.MHPlayerController|GetMHHUDWidget _asmhplayer_controller)))
          (Class|Image|SetOpacity (Variables|/Game/Characters/Utusi/UI/WBP_MonsterIcon.WBP_MonsterIcon_C|GetNargacugaIcon (Variables|/Game/Characters/Utusi/UI/WBP_MHHUD.WBP_MHHUD_C|GetWBP_MonsterIcon _aswbp_mhhud)) 0.5))
        (:OnFail
          (Development|PrintString "실패!"))))))

(fn ConstructionScript)

(fn GetGroundSpeed
  (return (Math|Vector|VectorLength (Variables|/Script/Engine.MovementComponent|GetVelocity (Variables|Character|GetCharacterMovement)))))