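; Trigger-box gimmick that starts a one-time turf war between Rathalos and Nargacuga when a player enters it.
; On overlap it spawns Nargacuga in front of Rathalos, facing it, and reveals the Nargacuga icon on the player's HUD.
; It then unpossesses Rathalos from its AI controller and plays the turf war montage, followed on completion by the dragon-ride-ready montage.
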(event OnComponentBeginOverlap(Box)
  (params (OverlappedComponent :type Primitive%20Component%20Object%20Reference) (OtherActor :type Actor%20Object%20Reference) (OtherComp :type Primitive%20Component%20Object%20Reference) (OtherBodyIndex :type Integer) (bFromSweep :type Boolean) (SweepResult :type Hit%20Result%20Structure%20%28by%20ref%29))
  ;[1 1 1] 나르가쿠르가 소환
  (if (and (not (Variables|Default|GetIsTriggered)) (Utilities|DoesObjectImplementInterface OtherActor "/Game/Blueprints/BPI_IsPlayer.BPI_IsPlayer_C"))
    (bind _returnvalue (Actor|GetActorOfClass "/Game/Blueprints/BP_MHCharacterRathalos.BP_MHCharacterRathalos_C"))
    (Game|SpawnActorfromClass "/Game/Blueprints/BP_MHCharacterNargacuga.BP_MHCharacterNargacuga_C" (Math|Transform|MakeTransform (+ (Transformation|GetActorLocation _returnvalue) (* (Transformation|GetActorForwardVector _returnvalue) 1.5e+03)) (Math|Conversions|RotationFromXVector (* (Transformation|GetActorForwardVector _returnvalue) -1.0)) "1.000000,1.000000,1.000000") "AdjustIfPossibleButAlwaysSpawn" 0 0)
    (Variables|Default|SetIsTriggered true)
    (bind _asmhplayer_controller (Utilities|Casting|CastToMHPlayerController (Game|GetPlayerController 0)))
    (bind _aswbp_mhhud (Utilities|Casting|CastToWBP_MHHUD (Variables|/Script/UERise.MHPlayerController|GetMHHUDWidget _asmhplayer_controller)))
    (Class|Image|SetOpacity (Variables|/Game/Characters/Utusi/UI/WBP_MonsterIcon.WBP_MonsterIcon_C|GetNargacugaIcon (Variables|/Game/Characters/Utusi/UI/WBP_MHHUD.WBP_MHHUD_C|GetWBP_MonsterIcon _aswbp_mhhud)) 1.0)
    ;[1 1 1] 리오레우스 영역다툼 몽타주 재생
    (bind _returnvalue_2 (Actor|GetActorOfClass "/Game/Blueprints/BP_MHCharacterRathalos.BP_MHCharacterRathalos_C"))
    (bind _output_get (Variables|Default|SetMonsterAIController (Pawn|GetController _returnvalue_2)))
    (Pawn|UnPossess _output_get)
    (Animation|Montage|PlayMontage (Variables|/Script/Engine.Character|GetMesh _returnvalue_2) "/Game/Animations/AM_TurfWar.AM_TurfWar"
      (:OnCompleted
        (Animation|Montage|PlayMontage (Variables|/Script/Engine.Character|GetMesh _returnvalue_2) "/Game/Animations/AM_DragonRideReady.AM_DragonRideReady")))))

(event EventBeginPlay)

(event Collision|EventActorBeginOverlap
  (params (OtherActor :type Actor%20Object%20Reference)))

(event EventTick
  (params (DeltaSeconds :type Float%20%28single-precision%29)))

(fn ConstructionScript)